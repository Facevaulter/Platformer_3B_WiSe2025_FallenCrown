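; Rune gate Blueprint that opens once three linked rune stones are all switched on.
; Tick checks the stones' IsOn flags every frame and calls Open while all three are set.
; Open plays a timeline whose track, scaled by an open depth, drives the cube's relative Z location to move the gate.
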(event Custom|Open
  (bind _newtrack_0 (Timeline|Timeline Play)
    (:Update
      (Transformation|SetRelativeLocation (Variables|Default|GetCube) (Math|Vector|MakeVector 0.0 0.0 (* _newtrack_0 (Variables|Default|GetOpenDeapth))) false false))))

(event EventTick
  (params (DeltaSeconds :type Float%20%28single-precision%29))
  (if (Math|Boolean|ANDBoolean (Variables|/Game/BP/BP_Runestone.BP_Runestone_C|GetIsOn (Variables|Default|GetRuneStone_0)) (Variables|/Game/BP/BP_Runestone.BP_Runestone_C|GetIsOn (Variables|Default|GetRuneStone_1)) (Variables|/Game/BP/BP_Runestone.BP_Runestone_C|GetIsOn (Variables|Default|GetRuneStone_2)))
    (CallFunction|Open)))

(fn ConstructionScript)