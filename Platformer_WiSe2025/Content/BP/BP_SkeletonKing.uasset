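; BP_SkeletonKing is the player character, with Enhanced Input camera-yaw-relative movement, look, ground-only sprint and a jump that requires re-pressing.
; Interact sphere-overlaps nearby actors and messages those implementing the interactable interface; Pause is forwarded to BP_Hud.
; BeginPlay moves it to the spawn transform saved in BP_GameInstance.
; Respawn runs once, fading out, teleporting to spawn, starting a fade-in and reopening the current level.
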(event Custom|Respawn
  (bind _returnvalue (Game|GetPlayerCameraManager 0))
  (Utilities|FlowControl|DoOnce false
    (:Completed
      (CameraFades|StartCameraFade :self _returnvalue :ToAlpha 1.0 :Duration 1.0 :bShouldFadeAudio true :bHoldWhenFinished true)
      (Utilities|FlowControl|Delay 1.0)
      (CallFunction|TeleporttoSpawn)
      (CameraFades|StartCameraFade :self _returnvalue :FromAlpha 1.0 :Duration 2.0 :bShouldFadeAudio true :bHoldWhenFinished true)
      (bind _returnvalue_2 (Game|GetCurrentLevelName true))
      (Game|OpenLevel(byName) (Utilities|String|StringToName _returnvalue_2)))))

(event Input|EnhancedActionEvents|EnhancedInputActionIA_Move
  (params (ActionValue :type Vector%202D%20Structure) (ElapsedSeconds :type Float%20%28double-precision%29) (TriggeredSeconds :type Float%20%28double-precision%29) (InputAction :type Input%20Action%20Object%20Reference :default "/Game/Input/Actions/IA_Move.IA_Move"))
  ;[0.01455 0.15 0.01847 0.5] Input
  (CallFunction|MoveinLocalDir (.x ActionValue) (.y ActionValue)))

(event Input|EnhancedActionEvents|EnhancedInputActionIA_Look
  (params (ActionValue :type Vector%202D%20Structure) (ElapsedSeconds :type Float%20%28double-precision%29) (TriggeredSeconds :type Float%20%28double-precision%29) (InputAction :type Input%20Action%20Object%20Reference :default "/Game/Input/Actions/IA_Look.IA_Look"))
  ;[0.01455 0.15 0.01847 0.5] Input
  (Pawn|Input|AddControllerYawInput (.x ActionValue))
  (Pawn|Input|AddControllerPitchInput (.y ActionValue)))

(event Input|EnhancedActionEvents|EnhancedInputActionIA_Jump
  (params (ActionValue :type Boolean) (ElapsedSeconds :type Float%20%28double-precision%29) (TriggeredSeconds :type Float%20%28double-precision%29) (InputAction :type Input%20Action%20Object%20Reference :default "/Game/Input/Actions/IA_Jump.IA_Jump"))
  ;[0.01455 0.15 0.01847 0.5] Input
  (:Triggered
    (if (not (Variables|Default|GetBunnyhopBreak))
      (Character|Jump)
      (Variables|Default|SetBunnyhopBreak true)))
  (:Completed
    (Character|StopJumping)
    (Variables|Default|SetBunnyhopBreak false)))

(event Input|EnhancedActionEvents|EnhancedInputActionIA_Sprint
  (params (ActionValue :type Boolean) (ElapsedSeconds :type Float%20%28double-precision%29) (TriggeredSeconds :type Float%20%28double-precision%29) (InputAction :type Input%20Action%20Object%20Reference :default "/Game/Input/Actions/IA_Sprint.IA_Sprint"))
  ;[0.01455 0.15 0.01847 0.5] Input
  (:Triggered
    (Variables|Default|SetWants%20to%20sprint true))
  (:Completed
    (Variables|Default|SetWants%20to%20sprint false)))

(event Input|EnhancedActionEvents|EnhancedInputActionIA_Interact
  (params (ActionValue :type Boolean) (ElapsedSeconds :type Float%20%28double-precision%29) (TriggeredSeconds :type Float%20%28double-precision%29) (InputAction :type Input%20Action%20Object%20Reference :default "/Game/Input/Actions/IA_Interact.IA_Interact"))
  (bind _interactsphere (Variables|Default|GetInteractSphere))
  ;[0.01455 0.15 0.01847 0.5] Input
  (bind _outactors (Collision|SphereOverlapActors (Transformation|GetWorldLocation _interactsphere) (Components|Sphere|GetScaledSphereRadius _interactsphere) (Utilities|Array|MakeArray "ObjectTypeQuery1" "ObjectTypeQuery2" "ObjectTypeQuery3") 0 (Utilities|Array|MakeArray self)))
  (for _array_element _outactors
    (if (Utilities|DoesObjectImplementInterface _array_element "/Game/BP/Interactions/InteractableInteraface.InteractableInteraface_C")
      (Class|InteractableInteraface|Interact(Message) _array_element))))

(event Input|EnhancedActionEvents|EnhancedInputActionIA_Pause
  (params (ActionValue :type Boolean) (ElapsedSeconds :type Float%20%28double-precision%29) (TriggeredSeconds :type Float%20%28double-precision%29) (InputAction :type Input%20Action%20Object%20Reference :default "/Game/Input/Actions/IA_Pause.IA_Pause"))
  ;[0.01455 0.15 0.01847 0.5] Input
  (bind _asbp_hud (Utilities|Casting|CastToBP_Hud (HUD|GetHUD (Game|GetPlayerController 0))))
  (Default|Pause _asbp_hud))

(event EventBeginPlay
  (CallFunction|TeleporttoSpawn)
  (Input|AddMappingContext (PlayerController|LocalPlayerSubsystems|GetEnhancedInputLocalPlayerSubsystem (Game|GetPlayerController 0)) "/Game/Input/IMC_Default.IMC_Default" 0 "(bIgnoreAllPressedKeysUntilRelease=True,bForceImmediately=False,bNotifyUserSettings=False)"))

(event EventTick
  (params (DeltaSeconds :type Float%20%28single-precision%29))
  (bind _charactermovement (Variables|Character|GetCharacterMovement))
  (if (and (Variables|Default|GetWants%20to%20sprint) (AI|Components|NavMovement|IsMovingonGround (Variables|Character|GetCharacterMovement)))
    (Variables|/Script/Engine.CharacterMovementComponent|SetMaxWalkSpeed _charactermovement (Variables|Default|GetSprintSpeed))
    (else
      (Variables|/Script/Engine.CharacterMovementComponent|SetMaxWalkSpeed _charactermovement (Variables|Default|GetWalkSpeed)))))

(fn ConstructionScript
  (Variables|/Script/Engine.CharacterMovementComponent|SetMaxWalkSpeed (Variables|Character|GetCharacterMovement) (Variables|Default|GetWalkSpeed)))

(fn MoveinLocalDir
  (params (LocalDirection_X :type Float%20%28double-precision%29) (LocalDirection_Y :type Float%20%28double-precision%29))
  (bind _camera (Variables|Default|GetCamera))
  (bind _returnvalue (Transformation|GetWorldTransform _camera))
  (Pawn|Input|AddMovementInput (Math|Transform|TransformDirection (Math|Transform|MakeTransform (.location _returnvalue) (Math|Rotator|MakeRotator 0.0 0.0 (.yaw (.rotation _returnvalue))) (.scale _returnvalue)) (Math|Vector|MakeVector LocalDirection_X LocalDirection_Y 0.0)) 1.0 false))

(fn TeleporttoSpawn
  (bind _asbp_game_instance (Utilities|Casting|CastToBP_GameInstance (Game|GetGameInstance))
    (:then
      (if (.HasValidPlayerSpawnTransform (Default|TryGetPlayerSpawnTransform _asbp_game_instance))
        (Transformation|SetActorLocationAndRotation (.location (.PlayerSpawnTransform (Default|TryGetPlayerSpawnTransform _asbp_game_instance))) (.rotation (.PlayerSpawnTransform (Default|TryGetPlayerSpawnTransform _asbp_game_instance))))))
    (:CastFailed
      (Development|PrintString "WRONG GAME INSTANCE" true true "(R=1.000000,G=0.019690,B=0.000000,A=1.000000)" 5.0))))