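; BP_SpikeTrap is a trap actor that shoots spikes out when a BP_Character enters its trigger box and respawns characters the spikes touch.
; Box overlap sets a re-trigger guard, waits a delay, then plays the ShootUP timeline to move the Spikes along local Z, clearing the guard when finished.
; Spikes overlap waits a death delay before calling Respawn on the character.
; BeginPlay derives the timeline play rate from SpikeSpeed.
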(event OnComponentBeginOverlap(Box)
  (params (OverlappedComponent :type Primitive%20Component%20Object%20Reference) (OtherActor :type Actor%20Object%20Reference) (OtherComp :type Primitive%20Component%20Object%20Reference) (OtherBodyIndex :type Integer) (bFromSweep :type Boolean) (SweepResult :type Hit%20Result%20Structure%20%28by%20ref%29))
  (Utilities|Casting|CastToBP_Character OtherActor)
  (if (not (Variables|Default|GetIsTriggert))
    (Variables|Default|SetIsTriggert true)
    (Utilities|FlowControl|Delay (Variables|Default|GetSpikeDelay))
    (bind _newtrack_0 (Timeline|ShootUP PlayFromStart)
      (:Update
        (Transformation|SetRelativeLocation (Variables|Default|GetSpikes) (Math|Vector|MakeVector 0.0 0.0 (* _newtrack_0 (Variables|Default|GetSpikeShootDistance))) false false))
      (:Finished
        (Variables|Default|SetIsTriggert false)))))

(event OnComponentBeginOverlap(Spikes)
  (params (OverlappedComponent :type Primitive%20Component%20Object%20Reference) (OtherActor :type Actor%20Object%20Reference) (OtherComp :type Primitive%20Component%20Object%20Reference) (OtherBodyIndex :type Integer) (bFromSweep :type Boolean) (SweepResult :type Hit%20Result%20Structure%20%28by%20ref%29))
  (bind _asbp_character (Utilities|Casting|CastToBP_Character OtherActor))
  (Utilities|FlowControl|Delay (Variables|Default|GetDeathDelay))
  (Default|Respawn _asbp_character))

(event EventBeginPlay
  (Components|Timeline|SetPlayRate (Variables|Default|GetShootUP) (/ 1.0 (Variables|Default|GetSpikeSpeed))))

(event Collision|EventActorBeginOverlap
  (params (OtherActor :type Actor%20Object%20Reference)))

(event EventTick
  (params (DeltaSeconds :type Float%20%28single-precision%29)))

(fn ConstructionScript)