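; BP_Door is a swinging door that opens automatically when a BP_Character enters either of its two trigger boxes.
; Each box sets an opposite swing direction and plays the OpenDoor timeline, and leaving either box reverses it.
; The timeline, rate-scaled by DoorSpeed, drives DoorPivot yaw up to MaxOpenAngle.
; A CanChangeDir flag locks the direction until the door is nearly closed, preventing mid-swing flips.
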(event OnComponentBeginOverlap(Box)
  (params (OverlappedComponent :type Primitive%20Component%20Object%20Reference) (OtherActor :type Actor%20Object%20Reference) (OtherComp :type Primitive%20Component%20Object%20Reference) (OtherBodyIndex :type Integer) (bFromSweep :type Boolean) (SweepResult :type Hit%20Result%20Structure%20%28by%20ref%29))
  (Utilities|Casting|CastToBP_Character OtherActor)
  (if (Variables|Default|GetCanChangeDir)
    (Variables|Default|SetOpenDir 1.0))
  (Variables|Default|SetCanChangeDir false)
  (bind _dooropenpercent (Timeline|OpenDoor Play)
    (:Update
      (Math|Float|CompareFloat _dooropenpercent 0.05
        (:>
          _)
        (:==
          (Variables|Default|SetCanChangeDir true :!label _label))
        (:<
          (goto _label)))
      (Transformation|SetRelativeRotation (Variables|Default|GetDoorPivot) (Math|Rotator|MakeRotator 0.0 0.0 (* _dooropenpercent (* (Variables|Default|GetMaxOpenAngle) (Variables|Default|GetOpenDir)))) false false))))

(event OnComponentEndOverlap(Box)
  (params (OverlappedComponent :type Primitive%20Component%20Object%20Reference) (OtherActor :type Actor%20Object%20Reference) (OtherComp :type Primitive%20Component%20Object%20Reference) (OtherBodyIndex :type Integer))
  (Utilities|Casting|CastToBP_Character OtherActor)
  (bind _dooropenpercent (Timeline|OpenDoor Reverse)
    (:Update
      (Math|Float|CompareFloat _dooropenpercent 0.05
        (:>
          _)
        (:==
          (Variables|Default|SetCanChangeDir true :!label _label))
        (:<
          (goto _label)))
      (Transformation|SetRelativeRotation (Variables|Default|GetDoorPivot) (Math|Rotator|MakeRotator 0.0 0.0 (* _dooropenpercent (* (Variables|Default|GetMaxOpenAngle) (Variables|Default|GetOpenDir)))) false false))))

(event OnComponentBeginOverlap(Box1)
  (params (OverlappedComponent :type Primitive%20Component%20Object%20Reference) (OtherActor :type Actor%20Object%20Reference) (OtherComp :type Primitive%20Component%20Object%20Reference) (OtherBodyIndex :type Integer) (bFromSweep :type Boolean) (SweepResult :type Hit%20Result%20Structure%20%28by%20ref%29))
  (Utilities|Casting|CastToBP_Character OtherActor)
  (if (Variables|Default|GetCanChangeDir)
    (Variables|Default|SetOpenDir -1.0))
  (Variables|Default|SetCanChangeDir false)
  (bind _dooropenpercent (Timeline|OpenDoor Play)
    (:Update
      (Math|Float|CompareFloat _dooropenpercent 0.05
        (:>
          _)
        (:==
          (Variables|Default|SetCanChangeDir true :!label _label))
        (:<
          (goto _label)))
      (Transformation|SetRelativeRotation (Variables|Default|GetDoorPivot) (Math|Rotator|MakeRotator 0.0 0.0 (* _dooropenpercent (* (Variables|Default|GetMaxOpenAngle) (Variables|Default|GetOpenDir)))) false false))))

(event OnComponentEndOverlap(Box1)
  (params (OverlappedComponent :type Primitive%20Component%20Object%20Reference) (OtherActor :type Actor%20Object%20Reference) (OtherComp :type Primitive%20Component%20Object%20Reference) (OtherBodyIndex :type Integer))
  (Utilities|Casting|CastToBP_Character OtherActor)
  (bind _dooropenpercent (Timeline|OpenDoor Reverse)
    (:Update
      (Math|Float|CompareFloat _dooropenpercent 0.05
        (:>
          _)
        (:==
          (Variables|Default|SetCanChangeDir true :!label _label))
        (:<
          (goto _label)))
      (Transformation|SetRelativeRotation (Variables|Default|GetDoorPivot) (Math|Rotator|MakeRotator 0.0 0.0 (* _dooropenpercent (* (Variables|Default|GetMaxOpenAngle) (Variables|Default|GetOpenDir)))) false false))))

(event EventBeginPlay
  (Components|Timeline|SetPlayRate (Variables|Default|GetOpenDoor) (/ 1.0 (Variables|Default|GetDoorSpeed))))

(fn ConstructionScript)