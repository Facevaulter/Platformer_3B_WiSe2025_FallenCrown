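; BP_RunePebble is a rock prop that glows brighter as the player approaches.
; It creates a dynamic material on the rock mesh, and a Sphere trigger flags when BP_Character is inside.
; While flagged, Tick scales emissive strength by the player's distance relative to the sphere radius, and leaving resets it to zero.
; A separate RotateRandowm event applies a random world rotation to the Pivot.
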(event OnComponentEndOverlap(Sphere)
  (params (OverlappedComponent :type Primitive%20Component%20Object%20Reference) (OtherActor :type Actor%20Object%20Reference) (OtherComp :type Primitive%20Component%20Object%20Reference) (OtherBodyIndex :type Integer))
  (Utilities|Casting|CastToBP_Character OtherActor)
  (Variables|Default|SetInRange false)
  (Rendering|Material|SetScalarParameterValue (Variables|Default|GetMID) "EmissiveStrenght" 0.0 :!class /Script/Engine.MaterialInstanceDynamic))

(event OnComponentBeginOverlap(Sphere)
  (params (OverlappedComponent :type Primitive%20Component%20Object%20Reference) (OtherActor :type Actor%20Object%20Reference) (OtherComp :type Primitive%20Component%20Object%20Reference) (OtherBodyIndex :type Integer) (bFromSweep :type Boolean) (SweepResult :type Hit%20Result%20Structure%20%28by%20ref%29))
  (bind _asbp_character (Utilities|Casting|CastToBP_Character OtherActor))
  (Variables|Default|SetInRange true))

(event Custom|RotateRandowm
  (Transformation|AddWorldRotation (Variables|Default|GetPivot) (Math|Rotator|MakeRotator (Math|Random|RandomFloatinRange 0.0 1.8e+02) (Math|Random|RandomFloatinRange 0.0 1.8e+02) (Math|Random|RandomFloatinRange 0.0 1.8e+02)) false false))

(event EventBeginPlay
  (bind _returnvalue (Rendering|Material|CreateDynamicMaterialInstance (Variables|Default|GetSM_Rock_003) 0 0 "None" :!class /Script/Engine.PrimitiveComponent))
  (Variables|Default|SetMID _returnvalue))

(event EventTick
  (params (DeltaSeconds :type Float%20%28single-precision%29))
  (if (Variables|Default|GetInRange)
    (Rendering|Material|SetScalarParameterValue (Variables|Default|GetMID) "EmissiveStrenght" (* (Variables|Default|GetMaxEmission) (- 1.0 (Math|Float|Clamp(Float) (/ (Math|Vector|VectorLength (- (Transformation|GetActorLocation (Game|Player|GetPlayerPawn 0)) (Transformation|GetActorLocation))) (Components|Sphere|GetScaledSphereRadius (Variables|Default|GetSphere)))))) :!class /Script/Engine.MaterialInstanceDynamic)))

(fn ConstructionScript)