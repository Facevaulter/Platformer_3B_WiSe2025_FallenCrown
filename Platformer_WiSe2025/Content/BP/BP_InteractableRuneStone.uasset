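; BP_InteractableRuneStone is an interactable rune stone that lights up when activated.
; BeginPlay creates a dynamic material instance on the mesh's first material slot.
; The first Interact plays a timeline that drives the material's emissive strength up to a configurable maximum, then sets IsOn when it finishes.
; A DoOnce with no reset makes the activation one-shot.
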(event EventBeginPlay
  (bind _returnvalue (Rendering|Material|CreateDynamicMaterialInstance (Variables|Default|GetMesh) 0 0 "None" :!class /Script/Engine.PrimitiveComponent))
  (Variables|Default|SetMID _returnvalue))

(event EventInteract
  (Utilities|FlowControl|DoOnce false
    (:Completed
      (bind _emission (Timeline|Timeline Play)
        (:Update
          (Rendering|Material|SetScalarParameterValue (Variables|Default|GetMID) "EmissiveStrenght" (* _emission (Variables|Default|GetMax%20Emissive%20Strenght)) :!class /Script/Engine.MaterialInstanceDynamic))
        (:Finished
          (Variables|Default|SetIsOn true))))))

(fn ConstructionScript)