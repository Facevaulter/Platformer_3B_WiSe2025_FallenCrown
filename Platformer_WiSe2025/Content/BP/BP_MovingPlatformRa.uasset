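; Moving platform that slides its mesh along an offset vector, either continuously or when BP_Character overlaps its trigger box.
; The move type selects one of three timelines (repeating linear, back-and-forth or accelerated), whose alpha scales the offset into a relative location.
; Play rates derive from a shared duration.
; When a run finishes, it restarts if set to always move, otherwise the mesh snaps back to its origin.
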(event OnComponentBeginOverlap(Box)
  (params (OverlappedComponent :type Primitive%20Component%20Object%20Reference) (OtherActor :type Actor%20Object%20Reference) (OtherComp :type Primitive%20Component%20Object%20Reference) (OtherBodyIndex :type Integer) (bFromSweep :type Boolean) (SweepResult :type Hit%20Result%20Structure%20%28by%20ref%29))
  (Utilities|Casting|CastToBP_Character OtherActor)
  (CallFunction|StartMoving))

(event Custom|StartMovingAccelarating
  (bind _location (Timeline|TimelineAccelated PlayFromStart)
    (:Update
      (CallFunction|Move _location))
    (:Finished
      (CallFunction|FinishMoving))))

(event Custom|StartMovingBackAndForth
  (bind _location (Timeline|TimelineBaF PlayFromStart)
    (:Update
      (CallFunction|Move _location))
    (:Finished
      (CallFunction|FinishMoving))))

(event Custom|StartMovingLinear
  (bind _location (Timeline|TimelineLinear PlayFromStart)
    (:Update
      (CallFunction|Move _location))
    (:Finished
      (CallFunction|FinishMoving))))

(event EventBeginPlay
  (bind _timeline_duration (Variables|Default|GetTimeline%20Duration))
  (bind _returnvalue (/ 1.0 _timeline_duration))
  (Components|Timeline|SetPlayRate (Variables|Default|GetTimelineBaF) _returnvalue)
  (Components|Timeline|SetPlayRate (Variables|Default|GetTimelineLinear) _returnvalue)
  (Components|Timeline|SetPlayRate (Variables|Default|GetTimelineAccelated) _returnvalue)
  (if (Variables|Default|GetAlwaysMove)
    (CallFunction|StartMoving)))

(fn ConstructionScript)

(fn Move
  (params (MovePercentage :type Float%20%28double-precision%29))
  (Transformation|SetRelativeLocation (Variables|Default|GetMesh) (* MovePercentage (Variables|Default|GetMoveDistanceV)) false false))

(fn StartMoving
  (if (not (Variables|Default|GetIsMoving))
    (Variables|Default|SetIsMoving true)
    (switch Utilities|FlowControl|Switch|SwitchonEPlatformMoveType (Variables|Default|GetPlatformMoveType)
      (:NewEnumerator0
        (CallFunction|StartMovingLinear))
      (:NewEnumerator1
        (CallFunction|StartMovingBackandForth))
      (:NewEnumerator2
        (CallFunction|StartMovingAccelarating)))))

(fn ResetMeshLocation
  (Transformation|SetRelativeLocation (Variables|Default|GetMesh) "0, 0, 0" false false))

(fn FinishMoving
  (Variables|Default|SetIsMoving false)
  (if (Variables|Default|GetAlwaysMove)
    (CallFunction|StartMoving)
    (else
      (CallFunction|ResetMeshLocation))))