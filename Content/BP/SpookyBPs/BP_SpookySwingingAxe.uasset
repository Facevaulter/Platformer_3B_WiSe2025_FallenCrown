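; Swinging axe trap with ghost and real-world versions that respawns BP_SkeletonKing on contact.
; Timelines ping-pong each pivot's roll between rotation limits at configurable rates, with a start delay for the ghost axe.
; The ghost axe always swings; the real one swings and kills through capsule overlaps only when RealIsHanging.
; When not hanging, both versions register their parts with SpookyAsset's visibility and collision arrays.
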(event OnComponentBeginOverlap(GhostAxeHead)
  (params (OverlappedComponent :type Primitive%20Component%20Object%20Reference) (OtherActor :type Actor%20Object%20Reference) (OtherComp :type Primitive%20Component%20Object%20Reference) (OtherBodyIndex :type Integer) (bFromSweep :type Boolean) (SweepResult :type Hit%20Result%20Structure%20%28by%20ref%29))
  (bind _asbp_skeleton_king (Utilities|Casting|CastToBP_SkeletonKing OtherActor))
  (Default|Respawn _asbp_skeleton_king))

(event OnComponentBeginOverlap(Capsule3)
  (params (OverlappedComponent :type Primitive%20Component%20Object%20Reference) (OtherActor :type Actor%20Object%20Reference) (OtherComp :type Primitive%20Component%20Object%20Reference) (OtherBodyIndex :type Integer) (bFromSweep :type Boolean) (SweepResult :type Hit%20Result%20Structure%20%28by%20ref%29))
  (Variables|Default|SetHitEventActor OtherActor)
  (if (Variables|Default|GetRealIsHanging)
    (bind _asbp_skeleton_king (Utilities|Casting|CastToBP_SkeletonKing (Variables|Default|GetHitEventActor)))
    (Default|Respawn _asbp_skeleton_king)))

(event OnComponentBeginOverlap(Capsule2)
  (params (OverlappedComponent :type Primitive%20Component%20Object%20Reference) (OtherActor :type Actor%20Object%20Reference) (OtherComp :type Primitive%20Component%20Object%20Reference) (OtherBodyIndex :type Integer) (bFromSweep :type Boolean) (SweepResult :type Hit%20Result%20Structure%20%28by%20ref%29))
  (Variables|Default|SetHitEventActor OtherActor)
  (if (Variables|Default|GetRealIsHanging)
    (bind _asbp_skeleton_king (Utilities|Casting|CastToBP_SkeletonKing (Variables|Default|GetHitEventActor)))
    (Default|Respawn _asbp_skeleton_king)))

(event OnComponentBeginOverlap(Capsule1)
  (params (OverlappedComponent :type Primitive%20Component%20Object%20Reference) (OtherActor :type Actor%20Object%20Reference) (OtherComp :type Primitive%20Component%20Object%20Reference) (OtherBodyIndex :type Integer) (bFromSweep :type Boolean) (SweepResult :type Hit%20Result%20Structure%20%28by%20ref%29))
  (Variables|Default|SetHitEventActor OtherActor)
  (if (Variables|Default|GetRealIsHanging)
    (bind _asbp_skeleton_king (Utilities|Casting|CastToBP_SkeletonKing (Variables|Default|GetHitEventActor)))
    (Default|Respawn _asbp_skeleton_king)))

(event OnComponentBeginOverlap(Capsule)
  (params (OverlappedComponent :type Primitive%20Component%20Object%20Reference) (OtherActor :type Actor%20Object%20Reference) (OtherComp :type Primitive%20Component%20Object%20Reference) (OtherBodyIndex :type Integer) (bFromSweep :type Boolean) (SweepResult :type Hit%20Result%20Structure%20%28by%20ref%29))
  (Variables|Default|SetHitEventActor OtherActor)
  (if (Variables|Default|GetRealIsHanging)
    (bind _asbp_skeleton_king (Utilities|Casting|CastToBP_SkeletonKing (Variables|Default|GetHitEventActor)))
    (Default|Respawn _asbp_skeleton_king)))

(event Custom|StartGhostAxeSwing
  (bind _newtrack_0 (Timeline|GhostAxeSwing PlayFromStart)
    (:Update
      (Transformation|SetRelativeRotation (Variables|Default|GetAxePivotGhost) (Math|Rotator|MakeRotator (+ (* _newtrack_0 (* (Variables|Default|GetGhostMaxRotation) 2.0)) (* (Variables|Default|GetGhostMaxRotation) -1.0)) 0.0 0.0) false false))
    (:Finished
      (Variables|Default|SetForewardGhost (not (Variables|Default|GetForewardGhost)))
      (if (Variables|Default|GetForewardGhost)
        (CallFunction|StartGhostAxeSwing)
        (else
          (CallFunction|ReverseGhostAxeSwing))))))

(event Custom|StartRreal%20Swing
  (bind _newtrack_0 (Timeline|RealAxeSwing PlayFromStart)
    (:Update
      (Transformation|SetRelativeRotation (Variables|Default|GetAxePivotReal) (Math|Rotator|MakeRotator (+ (* _newtrack_0 (* (Variables|Default|GetRealMaxRotation) 2.0)) (* (Variables|Default|GetRealMaxRotation) -1.0)) 0.0 0.0) false false))
    (:Finished
      (Variables|Default|SetForewardReal (not (Variables|Default|GetForewardReal)))
      (if (Variables|Default|GetForewardReal)
        (CallFunction|StartRrealSwing)
        (else
          (CallFunction|ReverseRealSwing))))))

(event Custom|ReverseGhostAxeSwing
  (bind _newtrack_0 (Timeline|GhostAxeSwing ReverseFromEnd)
    (:Update
      (Transformation|SetRelativeRotation (Variables|Default|GetAxePivotGhost) (Math|Rotator|MakeRotator (+ (* _newtrack_0 (* (Variables|Default|GetGhostMaxRotation) 2.0)) (* (Variables|Default|GetGhostMaxRotation) -1.0)) 0.0 0.0) false false))
    (:Finished
      (Variables|Default|SetForewardGhost (not (Variables|Default|GetForewardGhost)))
      (if (Variables|Default|GetForewardGhost)
        (CallFunction|StartGhostAxeSwing)
        (else
          (CallFunction|ReverseGhostAxeSwing))))))

(event Custom|ReverseRealSwing
  (bind _newtrack_0 (Timeline|RealAxeSwing ReverseFromEnd)
    (:Update
      (Transformation|SetRelativeRotation (Variables|Default|GetAxePivotReal) (Math|Rotator|MakeRotator (+ (* _newtrack_0 (* (Variables|Default|GetRealMaxRotation) 2.0)) (* (Variables|Default|GetRealMaxRotation) -1.0)) 0.0 0.0) false false))
    (:Finished
      (Variables|Default|SetForewardReal (not (Variables|Default|GetForewardReal)))
      (if (Variables|Default|GetForewardReal)
        (CallFunction|StartRrealSwing)
        (else
          (CallFunction|ReverseRealSwing))))))

(event EventBeginPlay
  (bind _spookyasset (Variables|Default|GetSpookyAsset))
  (bind _realtaxehead (Variables|Default|GetRealtAxeHead))
  (bind _realworldactorarray_collision (Variables|/Game/BP/Components/SpookyAsset_Component.SpookyAsset_Component_C|GetRealWorldActorArray_Collision _spookyasset))
  (Utilities|FlowControl|Sequence
    (:then_0
      (if (not (Variables|Default|GetRealIsHanging))
        (Utilities|FlowControl|Sequence
          (:then_0
            (Utilities|Array|Add (Variables|/Game/BP/Components/SpookyAsset_Component.SpookyAsset_Component_C|GetGhostActorArray_Visibility _spookyasset) (Variables|Default|GetGhost))
            (Utilities|Array|Add (Variables|/Game/BP/Components/SpookyAsset_Component.SpookyAsset_Component_C|GetGhostActorArray_Collision _spookyasset) (Variables|Default|GetGhostAxeStikMesh))
            (Utilities|Array|Add (Variables|/Game/BP/Components/SpookyAsset_Component.SpookyAsset_Component_C|GetGhostActorArray_ComplexOverlap _spookyasset) (Variables|Default|GetGhostAxeHead)))
          (:then_1
            (Utilities|Array|Add (Variables|/Game/BP/Components/SpookyAsset_Component.SpookyAsset_Component_C|GetRealWorldActorArray_Visibility _spookyasset) (Variables|Default|GetReal))
            (Utilities|Array|Add _realworldactorarray_collision (Variables|Default|GetRealAxeStikMesh1))
            (Utilities|Array|Add _realworldactorarray_collision (Variables|Default|GetRealtAxeHead))))))
    (:then_1
      (Components|Timeline|SetPlayRate (Variables|Default|GetGhostAxeSwing) (/ 1.0 (Variables|Default|GetGhostAxeSwingPlayrate)))
      (Components|Timeline|SetPlayRate (Variables|Default|GetRealAxeSwing) (/ 1.0 (Variables|Default|GetRealAxeSwingPlayrate))))
    (:then_2
      (Utilities|FlowControl|Sequence
        (:then_0
          (if (Variables|Default|GetRealIsHanging)
            (Utilities|FlowControl|Sequence
              (:then_0
                (Collision|SetCollisionEnabled _realtaxehead "NoCollision")
                (Variables|/Script/Engine.PrimitiveComponent|SetbGenerateOverlapEvents _realtaxehead true))
              (:then_1
                (bind _result (Math|Float|NegateFloat (Variables|Default|GetRealMaxRotation))
                  (:%20%20
                    (Transformation|SetRelativeRotation (Variables|Default|GetAxePivotReal) (Math|Rotator|MakeRotator _result 0.0 0.0) false false)
                    (CallFunction|StartRrealSwing)))))))
        (:then_1
          (bind _result_2 (Math|Float|NegateFloat (Variables|Default|GetGhostMaxRotation))
            (:%20%20
              (Transformation|SetRelativeRotation (Variables|Default|GetAxePivotGhost) (Math|Rotator|MakeRotator _result_2 0.0 0.0) false false)
              (Utilities|FlowControl|Delay (Variables|Default|GetGhostStartDelay))
              (CallFunction|StartGhostAxeSwing))))))))

(fn ConstructionScript)