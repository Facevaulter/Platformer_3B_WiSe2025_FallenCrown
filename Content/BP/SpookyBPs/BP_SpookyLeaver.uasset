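; BP_SpookyLeaver is an interactable lever that opens a linked gate and moves the player's ghost wind guide to the next target.
; Its optional ghost variant swaps visibility through SpookyAssetComponent and only responds or shows the HUD prompt in the ghost realm.
; Interacting plays a sound, enables the next wind target's overlaps, and runs a one-shot rotation timeline that opens the gate when finished.
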(event OnComponentBeginOverlap(InteractHudCheck)
  (params (OverlappedComponent :type Primitive%20Component%20Object%20Reference) (OtherActor :type Actor%20Object%20Reference) (OtherComp :type Primitive%20Component%20Object%20Reference) (OtherBodyIndex :type Integer) (bFromSweep :type Boolean) (SweepResult :type Hit%20Result%20Structure%20%28by%20ref%29))
  (Utilities|Casting|CastToBP_SkeletonKing OtherActor)
  (if (Variables|Default|GetUseGhostLeaver)
    (if (Variables|/Game/BP/Components/SpookyAsset_Component.SpookyAsset_Component_C|GetInGhostRealm (Variables|Default|GetSpookyAsset_Component))
      (bind _asbp_hud (Utilities|Casting|CastToBP_Hud (HUD|GetHUD (Game|GetPlayerController 0)) :!label _label))
      (Default|ShowInteractTxt (Variables|/Game/UI/BP_Hud.BP_Hud_C|GetInteractWidget _asbp_hud)))
    (else
      (goto _label))))

(event OnComponentEndOverlap(InteractHudCheck)
  (params (OverlappedComponent :type Primitive%20Component%20Object%20Reference) (OtherActor :type Actor%20Object%20Reference) (OtherComp :type Primitive%20Component%20Object%20Reference) (OtherBodyIndex :type Integer))
  (Utilities|Casting|CastToBP_SkeletonKing OtherActor)
  (bind _asbp_hud (Utilities|Casting|CastToBP_Hud (HUD|GetHUD (Game|GetPlayerController 0))))
  (Default|HideInteractTxt (Variables|/Game/UI/BP_Hud.BP_Hud_C|GetInteractWidget _asbp_hud)))

(event Custom|StartLeaverDown
  (Utilities|FlowControl|DoOnce false
    (:Completed
      (bind _newtrack_0 (Timeline|LeaverDownTImeline PlayFromStart)
        (:Update
          (Transformation|SetRelativeRotation (Variables|Default|GetLeaverPivotToRotate) (Math|Rotator|MakeRotator (* _newtrack_0 (Variables|Default|GetMaxRotation)) 0.0 0.0) false false))
        (:Finished
          (Default|OpenGate (Variables|Default|GetGateToOpen)))))))

(event EventBeginPlay
  (bind _spookyasset_component (Variables|Default|GetSpookyAsset_Component))
  (Utilities|FlowControl|Sequence
    (:then_0
      (if (Variables|Default|GetUseGhostLeaver)
        (Variables|Default|SetLeaverPivotToRotate (Variables|Default|GetGhost%20Leaver%20Pivot))
        (Utilities|FlowControl|Sequence
          (:then_0
            (Utilities|Array|Add (Variables|/Game/BP/Components/SpookyAsset_Component.SpookyAsset_Component_C|GetGhostActorArray_Visibility _spookyasset_component) (Variables|Default|GetGhost)))
          (:then_1
            (Utilities|Array|Add (Variables|/Game/BP/Components/SpookyAsset_Component.SpookyAsset_Component_C|GetRealWorldActorArray_Visibility _spookyasset_component) (Variables|Default|GetRealLeaver))))
        (else
          (Variables|Default|SetLeaverPivotToRotate (Variables|Default|GetRealPivot)))))))

(event EventInteract
  (if (Variables|Default|GetUseGhostLeaver)
    (if (Variables|/Game/BP/Components/SpookyAsset_Component.SpookyAsset_Component_C|GetInGhostRealm (Variables|Default|GetSpookyAsset_Component))
      (CallFunction|StartLeaverDown :!label _label)
      (Audio|PlaySoundatLocation "/Game/Audio/Sfx/LeaverSFX.LeaverSFX" (Transformation|GetActorLocation) "0, 0, 0" 1.0 1.0 0.0 "/Game/Audio/Sfx/SpikeTrap_AttenuationSetting.SpikeTrap_AttenuationSetting" 0 0 0)
      (bind _asbp_skeleton_king (Utilities|Casting|CastToBP_SkeletonKing (Game|GetPlayerCharacter 0)))
      (Variables|/Game/BP/BP_SkeletonKing.BP_SkeletonKing_C|SetGhostWIndTarget _asbp_skeleton_king (Transformation|GetActorLocation (Variables|Default|GetNextWindTarget)))
      (Development|PrintString "SetNewWindTarget")
      (bind _asbp_ghost_wind_target (Utilities|Casting|CastToBP_GhostWindTarget (Variables|Default|GetNextWindTarget)))
      (Variables|/Script/Engine.PrimitiveComponent|SetbGenerateOverlapEvents (Variables|/Game/BP/BP_GhostWindTarget.BP_GhostWindTarget_C|GetSphere _asbp_ghost_wind_target) true)
      (Development|PrintString "Set New Target" true true "(R=0.000000,G=0.660000,B=1.000000,A=1.000000)" 3.0)
      (Development|PrintString (Utilities|String|ToString(Object) _asbp_ghost_wind_target) true true "(R=0.000000,G=0.660000,B=1.000000,A=1.000000)" 3.0))
    (else
      (goto _label))))

(fn ConstructionScript)