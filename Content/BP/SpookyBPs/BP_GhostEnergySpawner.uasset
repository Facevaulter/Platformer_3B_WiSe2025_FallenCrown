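; Spawner actor that places a BP_GhostEnergy actor at its root location and replaces it on respawn.
; On BeginPlay it casts the player character to BP_SkeletonKing, binds to its RespawnGhostEnergy dispatcher and spawns the first instance.
; SpawnGhostEnergy reuses that spawn logic only when the stored instance is no longer valid, so each spawner avoids duplicates.
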(event Custom|SpawnGhostEnergy
  (Variables|Default|GetSpawned%20coin
    (:then)
    (:else
      (bind _returnvalue (Game|SpawnActorfromClass "/Game/BP/Collectibles/BP_GhostEnergy.BP_GhostEnergy_C" (Math|Transform|MakeTransform (Transformation|GetWorldLocation (Variables|Default|GetDefaultSceneRoot)) "0, 0, 0" "1.000000,1.000000,1.000000") "Undefined" "MultiplyWithRoot" 0 0))
      (Variables|Default|SetSpawned%20coin _returnvalue))))

(event EventBeginPlay
  (bind _asbp_skeleton_king (Utilities|Casting|CastToBP_SkeletonKing (Game|GetPlayerCharacter 0)))
  (Variables|Default|SetDispatcher%20Ref _asbp_skeleton_king)
  (bind _dispatcher_ref (Variables|Default|GetDispatcher%20Ref)
    (:then
      (EventDispatchers|BindEventtoRespawnGhostEnergy _dispatcher_ref (EventDispatchers|CreateEvent :!event Custom|SpawnGhostEnergy))
      (bind _returnvalue (Game|SpawnActorfromClass "/Game/BP/Collectibles/BP_GhostEnergy.BP_GhostEnergy_C" (Math|Transform|MakeTransform (Transformation|GetWorldLocation (Variables|Default|GetDefaultSceneRoot)) "0, 0, 0" "1.000000,1.000000,1.000000") "Undefined" "MultiplyWithRoot" 0 0))
      (Variables|Default|SetSpawned%20coin _returnvalue))
    (:else)))

(fn ConstructionScript)