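; BP_MovingGhostPlatform is a platform with ghost and real-world forms, registered with SpookyAsset for world toggling, where only the ghost mesh moves.
; Movement starts on BeginPlay if set to always move, or when BP_SkeletonKing overlaps the ghost box, unless NothingMoves is set.
; The move type picks one of three duration-scaled timelines (linear, back-and-forth, accelerated) driving the mesh's relative offset.
; On finish it restarts if always moving, otherwise snaps back to origin.
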(event OnComponentBeginOverlap(GhostBox)
  (params (OverlappedComponent :type Primitive%20Component%20Object%20Reference) (OtherActor :type Actor%20Object%20Reference) (OtherComp :type Primitive%20Component%20Object%20Reference) (OtherBodyIndex :type Integer) (bFromSweep :type Boolean) (SweepResult :type Hit%20Result%20Structure%20%28by%20ref%29))
  ;[0.15 0.15 0.15 0.5] Player stepped on Platform
  (Utilities|Casting|CastToBP_SkeletonKing OtherActor)
  (if (not (Variables|Default|GetNothingMoves))
    (CallFunction|StartMoving)))

(event Custom|StartMovingAccelarating
  ;[0.15 0.15 0.15 0.5] Movement Timelines
  (bind _location (Timeline|TimelineAccelated PlayFromStart)
    (:Update
      (CallFunction|Move _location))
    (:Finished
      (CallFunction|FinishMoving))))

(event Custom|StartMovingBackAndForth
  ;[0.15 0.15 0.15 0.5] Movement Timelines
  (bind _location (Timeline|TimelineBaF PlayFromStart)
    (:Update
      (CallFunction|Move _location))
    (:Finished
      (CallFunction|FinishMoving))))

(event Custom|StartMovingLinear
  ;[0.15 0.15 0.15 0.5] Movement Timelines
  (bind _location (Timeline|TimelineLinear PlayFromStart)
    (:Update
      (CallFunction|Move _location))
    (:Finished
      (CallFunction|FinishMoving))))

(event EventBeginPlay
  (bind _spookyasset (Variables|Default|GetSpookyAsset))
  (bind _timeline_duration (Variables|Default|GetTimeline%20Duration))
  (bind _returnvalue (/ 1.0 _timeline_duration))
  (Utilities|FlowControl|Sequence
    (:then_0
      ;[0.15 0.15 0.15 0.5] Ghost Toggle Setup
      (Utilities|FlowControl|Sequence
        (:then_0
          (Utilities|Array|Add (Variables|/Game/BP/Components/SpookyAsset_Component.SpookyAsset_Component_C|GetGhostActorArray_Visibility _spookyasset) (Variables|Default|GetGhostForm))
          (Utilities|Array|Add (Variables|/Game/BP/Components/SpookyAsset_Component.SpookyAsset_Component_C|GetGhostActorArray_TriggerBox _spookyasset) (Variables|Default|GetGhostBox))
          (Utilities|Array|Add (Variables|/Game/BP/Components/SpookyAsset_Component.SpookyAsset_Component_C|GetGhostActorArray_Collision _spookyasset) (Variables|Default|GetGhostMesh)))
        (:then_1
          (Utilities|Array|Add (Variables|/Game/BP/Components/SpookyAsset_Component.SpookyAsset_Component_C|GetRealWorldActorArray_Visibility _spookyasset) (Variables|Default|GetRealForm))
          (Utilities|Array|Add (Variables|/Game/BP/Components/SpookyAsset_Component.SpookyAsset_Component_C|GetRealWorldActorArray_TriggerBox _spookyasset) (Variables|Default|GetRealBox1))
          (Utilities|Array|Add (Variables|/Game/BP/Components/SpookyAsset_Component.SpookyAsset_Component_C|GetRealWorldActorArray_Collision _spookyasset) (Variables|Default|GetRealMesh1)))))
    (:then_1
      (if (not (Variables|Default|GetNothingMoves))
        ;[0.15 0.15 0.15 0.5] Set Movespeed
        (Components|Timeline|SetPlayRate (Variables|Default|GetTimelineBaF) _returnvalue)
        (Components|Timeline|SetPlayRate (Variables|Default|GetTimelineLinear) _returnvalue)
        (Components|Timeline|SetPlayRate (Variables|Default|GetTimelineAccelated) _returnvalue)
        (if (Variables|Default|GetGhostAlwaysMove)
          ;[0.15 0.15 0.15 0.5] Start Moving
          (CallFunction|StartMoving))))))

(fn ConstructionScript)

(fn Move
  (params (MovePercentage :type Float%20%28double-precision%29))
  (Transformation|SetRelativeLocation (Variables|Default|GetGhostMesh) (* MovePercentage (- (Variables|Default|GetMoveDistanceVGhost) (Variables|/Script/Engine.SceneComponent|GetRelativeLocation (Variables|Default|GetGhostForm)))) false false))

(fn StartMoving
  (if (not (Variables|Default|GetGhostIsMoving))
    (Variables|Default|SetGhostIsMoving true)
    (switch Utilities|FlowControl|Switch|SwitchonEPlatformMoveType (Variables|Default|GetPlatformMoveTypeGhost)
      (:NewEnumerator0
        (CallFunction|StartMovingLinear))
      (:NewEnumerator1
        (CallFunction|StartMovingBackandForth))
      (:NewEnumerator2
        (CallFunction|StartMovingAccelarating)))))

(fn ResetMeshLocation
  (Transformation|SetRelativeLocation (Variables|Default|GetGhostMesh) "0, 0, 0" false false))

(fn FinishMoving
  (Variables|Default|SetGhostIsMoving false)
  (if (Variables|Default|GetGhostAlwaysMove)
    (CallFunction|StartMoving)
    (else
      (CallFunction|ResetMeshLocation))))