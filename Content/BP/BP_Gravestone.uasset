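; Gravestone actor that varies its own appearance at random when play begins.
; BeginPlay shifts the Cube mesh vertically and rotates it on all three axes within variable-set limits, then uniformly scales the Scene component by a random percentage around full size.
; It then picks one of three placeholder meshes (triangle, cone or cylinder) for Cube.
; The construction script is empty, so the variation appears only at runtime.
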(event EventBeginPlay
  (bind _cube (Variables|Default|GetCube))
  (bind _maxheightoffset (Variables|Default|GetMaxHeightOffset))
  (bind _maxrotationx (Variables|Default|GetMaxRotationX))
  (bind _maxrotationy (Variables|Default|GetMaxRotationY))
  (bind _maxscalein_ (Variables|Default|GetMaxScaleIn%25))
  (bind _maxrotationz (Variables|Default|GetMaxRotationZ))
  (bind _returnvalue (/ _maxscalein_ 1e+02))
  ;[0.15 0.15 0.15 0.5] Zufällige r Offset (Z-Achse)
  (Transformation|AddWorldOffset _cube (Math|Vector|MakeVector 0.0 0.0 (Math|Random|RandomFloatinRange (* _maxheightoffset -1.0) _maxheightoffset)) false false)
  ;[0.15 0.15 0.15 0.5] Zufällige Rotation (Z-Achse) und Zufällige Neigung(X-Achse & Y-Achse)
  (Transformation|AddWorldRotation _cube (Math|Rotator|MakeRotator (Math|Random|RandomFloatinRange (* _maxrotationx -1.0) _maxrotationx) (Math|Random|RandomFloatinRange (* _maxrotationy -1.0) _maxrotationy) (Math|Random|RandomFloatinRange (* _maxrotationz -1.0) _maxrotationz)) false false)
  ;[0.15 0.15 0.15 0.5] Zufällige Größe(20% größer oder kleiner)
  (Transformation|SetWorldScale3D (Variables|Default|GetScene) (Math|Conversions|ToVector(Float) (Math|Random|RandomFloatinRange (- 1.0 _returnvalue) (+ _returnvalue 1.0))))
  ;[0.15 0.15 0.15 0.5] Bonus: Assign random mesh (3 possible variants)
  (Math|Integer|CompareInt (Math|Random|RandomIntegerinRange 0 2) 1
    (:>
      (Components|StaticMesh|SetStaticMesh (Variables|Default|GetCube) "/ControlRig/Controls/ControlRig_Triangle_solid.ControlRig_Triangle_solid"))
    (:==
      (Components|StaticMesh|SetStaticMesh (Variables|Default|GetCube) "/Engine/BasicShapes/Cone.Cone"))
    (:<
      (Components|StaticMesh|SetStaticMesh (Variables|Default|GetCube) "/Engine/EngineMeshes/Cylinder.Cylinder"))))

(event Collision|EventActorBeginOverlap
  (params (OtherActor :type Actor%20Object%20Reference)))

(event EventTick
  (params (DeltaSeconds :type Float%20%28single-precision%29)))

(fn ConstructionScript)