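; BP_SpikeTrap is a spike trap that respawns BP_SkeletonKing when it overlaps Box1.
; The ShootUP timeline drives spike height, with speed and distance set by variables.
; It runs in three modes: always extended, self-repeating on an interval, or fired after a delay when the king enters Box.
; Interval mode disables Box overlaps, while triggered mode uses a flag to block retriggering until the timeline finishes.
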(event OnComponentBeginOverlap(Box1)
  (params (OverlappedComponent :type Primitive%20Component%20Object%20Reference) (OtherActor :type Actor%20Object%20Reference) (OtherComp :type Primitive%20Component%20Object%20Reference) (OtherBodyIndex :type Integer) (bFromSweep :type Boolean) (SweepResult :type Hit%20Result%20Structure%20%28by%20ref%29))
  (bind _asbp_skeleton_king (Utilities|Casting|CastToBP_SkeletonKing OtherActor))
  (Default|Respawn _asbp_skeleton_king))

(event OnComponentBeginOverlap(Box)
  (params (OverlappedComponent :type Primitive%20Component%20Object%20Reference) (OtherActor :type Actor%20Object%20Reference) (OtherComp :type Primitive%20Component%20Object%20Reference) (OtherBodyIndex :type Integer) (bFromSweep :type Boolean) (SweepResult :type Hit%20Result%20Structure%20%28by%20ref%29))
  (Utilities|Casting|CastToBP_SkeletonKing OtherActor)
  (if (not (Variables|Default|GetAlwaysExtended))
    (if (not (Variables|Default|GetIsTriggert))
      (Variables|Default|SetIsTriggert true)
      (Utilities|FlowControl|Delay (Variables|Default|GetSpikeDelay))
      (bind _newtrack_0 (Timeline|ShootUP PlayFromStart)
        (:Update
          (Transformation|SetRelativeLocation (Variables|Default|GetSpikes) (Math|Vector|MakeVector 0.0 0.0 (* _newtrack_0 (Variables|Default|GetSpikeShootDistance))) false false))
        (:Finished
          (if (Variables|Default|GetOnInterval)
            (Utilities|FlowControl|Delay (Variables|Default|GetAutoModePauseTime))
            (CallFunction|AutoActivate)
            (else
              (Variables|Default|SetIsTriggert false))))))))

(event Custom|AutoActivate
  (bind _newtrack_0 (Timeline|ShootUP PlayFromStart)
    (:Update
      (Transformation|SetRelativeLocation (Variables|Default|GetSpikes) (Math|Vector|MakeVector 0.0 0.0 (* _newtrack_0 (Variables|Default|GetSpikeShootDistance))) false false))
    (:Finished
      (if (Variables|Default|GetOnInterval)
        (Utilities|FlowControl|Delay (Variables|Default|GetAutoModePauseTime))
        (CallFunction|AutoActivate)
        (else
          (Variables|Default|SetIsTriggert false))))))

(event EventBeginPlay
  (if (Variables|Default|GetAlwaysExtended)
    (Transformation|SetRelativeLocation (Variables|Default|GetSpikes) (Math|Vector|MakeVector 0.0 0.0 (Variables|Default|GetSpikeShootDistance)) false false)
    (else
      (Components|Timeline|SetPlayRate (Variables|Default|GetShootUP) (/ 1.0 (Variables|Default|GetSpikeSpeed)))
      (if (Variables|Default|GetOnInterval)
        (Variables|/Script/Engine.PrimitiveComponent|SetbGenerateOverlapEvents (Variables|Default|GetBox) false)
        (Utilities|FlowControl|Delay (Variables|Default|GetAutoActivationDelay))
        (CallFunction|AutoActivate)))))

(fn ConstructionScript)