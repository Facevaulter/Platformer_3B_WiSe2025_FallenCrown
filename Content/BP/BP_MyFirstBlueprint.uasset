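; BP_MyFirstBlueprint is a practice actor with an animated mesh and a flickering, color-changing point light.
; BeginPlay offsets and rotates the mesh, resets its scale and swaps it to a pyramid.
; Tick raises it using delta time and spins it per frame, while chained Delays throttle random light intensity and, less often, random HSV color.
; Overlap and hit events are empty.
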(event EventBeginPlay
  (bind (_outputpin _outputpin2) (CallFunction|ModifyMesh)))

(event Collision|EventActorBeginOverlap
  (params (OtherActor :type Actor%20Object%20Reference))
  ;[0.04743 0.06526 0.15 0.5] Trigger and Collision
)

(event EventTick
  (params (DeltaSeconds :type Float%20%28single-precision%29))
  (bind _pointlight (Variables|Default|GetPointLight))
  (CallFunction|ModyfyLocation (stale EventBeginPlay _outputpin) (stale EventBeginPlay _outputpin2) DeltaSeconds)
  (Utilities|FlowControl|Delay 0.2)
  (CallFunction|RandomIntensity _pointlight)
  (Utilities|FlowControl|Delay 0.4)
  (CallFunction|RandomColor _pointlight))

(event Collision|EventHit
  (params (MyComp :type Primitive%20Component%20Object%20Reference) (Other :type Actor%20Object%20Reference) (OtherComp :type Primitive%20Component%20Object%20Reference) (bSelfMoved :type Boolean) (HitLocation :type Vector :default "0, 0, 0") (HitNormal :type Vector :default "0, 0, 0") (NormalImpulse :type Vector :default "0, 0, 0") (Hit :type Hit%20Result%20Structure%20%28by%20ref%29))
  ;[0.04743 0.06526 0.15 0.5] Trigger and Collision
)

(fn ConstructionScript)

(fn ModifyMesh
  (bind _mesh (Variables|Default|GetMesh))
  (Transformation|AddWorldOffset _mesh "0.000000,0.000000,100.000000" false false)
  (Transformation|AddLocalRotation _mesh "-90.000000,45.000000,0.000000" false false)
  (Transformation|SetRelativeScale3D _mesh "1.000000,1.000000,1.000000")
  (Components|StaticMesh|SetStaticMesh _mesh "/ControlRig/Controls/ControlRig_Pyramid_3mm.ControlRig_Pyramid_3mm")
  (return _mesh _mesh))

(fn ModyfyLocation
  (params (self2 :type Scene%20Component%20Object%20Reference) (self3 :type Scene%20Component%20Object%20Reference) (B :type Float%20%28single-precision%29))
  (Transformation|AddWorldOffset self2 (* "0.000000,0.000000,20.000000" B) false false)
  (Transformation|AddWorldRotation self3 "0.000000,3.000000,0.000000" false false))

(fn RandomColor
  (params (InputPin :type Point%20Light%20Component%20Object%20Reference))
  (Rendering|Components|Light|SetLightColor InputPin (Class|KismetMathLibrary|HSVtoRGB (Math|Random|RandomFloatinRange 0.0 3.6e+02) (Math|Random|RandomFloatinRange 0.0 1.0) (Math|Random|RandomFloatinRange 0.0 1.0) 1.0) true))

(fn RandomIntensity
  (params (self2 :type Light%20Component%20Object%20Reference))
  (Rendering|Components|Light|SetIntensity self2 (Math|Random|RandomFloatinRange (Variables|Light|GetLightIntensity_Min) (Variables|Light|GetLightIntensity_Max))))