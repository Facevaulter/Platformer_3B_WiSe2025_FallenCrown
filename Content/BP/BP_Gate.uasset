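; BP_Gate is a double stone gate that swings open and records its open state per gate in BP_GameInstance.
; OpenGate saves WhichGate as open, plays the stone door audio, then runs a one-shot timeline that yaws the two door pivots in opposite directions up to MaxRotation.
; LoadOpenGate enters the same DoOnce and animation directly, opening the gate without saving or sound.
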(event Custom|LoadOpenGate
  (Utilities|FlowControl|DoOnce false
    (:Completed
      (bind _newtrack_0 (Timeline|Timeline PlayFromStart)
        (:Update
          (Transformation|SetRelativeRotation (Variables|Default|GetPivotDoorR) (Math|Rotator|MakeRotator 0.0 0.0 (* _newtrack_0 (Variables|Default|GetMax%20Rotation))) false false)
          (Transformation|SetRelativeRotation (Variables|Default|GetPivotDoorL) (Math|Rotator|MakeRotator 0.0 0.0 (* (* _newtrack_0 (Variables|Default|GetMax%20Rotation)) -1.0)) false false))))))

(event Custom|OpenGate
  (bind _asbp_game_instance (Utilities|Casting|CastToBP_GameInstance (Game|GetGameInstance)))
  (Default|SaveGateOpen _asbp_game_instance (Variables|Default|GetWhichGate))
  (Audio|Components|Audio|Play (Variables|Default|GetAudioComponent_StoneDoor) 0.0)
  (Utilities|FlowControl|DoOnce false
    (:Completed
      (bind _newtrack_0 (Timeline|Timeline PlayFromStart)
        (:Update
          (Transformation|SetRelativeRotation (Variables|Default|GetPivotDoorR) (Math|Rotator|MakeRotator 0.0 0.0 (* _newtrack_0 (Variables|Default|GetMax%20Rotation))) false false)
          (Transformation|SetRelativeRotation (Variables|Default|GetPivotDoorL) (Math|Rotator|MakeRotator 0.0 0.0 (* (* _newtrack_0 (Variables|Default|GetMax%20Rotation)) -1.0)) false false))))))

(fn ConstructionScript)