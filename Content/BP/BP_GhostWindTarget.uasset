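; BP_GhostWindTarget is a chained waypoint that steers the Skeleton King's ghost wind target from one point to the next.
; On the first overlap of its sphere, a Skeleton King has its GhostWIndTarget set to the location of NextWindTarget, with a debug print.
; The waypoint then enables overlap events on the next BP_GhostWindTarget's sphere and disables its own, handing the trigger along the chain.
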(event OnComponentBeginOverlap(Sphere)
  (params (OverlappedComponent :type Primitive%20Component%20Object%20Reference) (OtherActor :type Actor%20Object%20Reference) (OtherComp :type Primitive%20Component%20Object%20Reference) (OtherBodyIndex :type Integer) (bFromSweep :type Boolean) (SweepResult :type Hit%20Result%20Structure%20%28by%20ref%29))
  (Utilities|FlowControl|DoOnce false
    (:Completed
      (bind _asbp_skeleton_king (Utilities|Casting|CastToBP_SkeletonKing OtherActor))
      (Variables|/Game/BP/BP_SkeletonKing.BP_SkeletonKing_C|SetGhostWIndTarget _asbp_skeleton_king (Transformation|GetActorLocation (Variables|Default|GetNextWindTarget)))
      (Development|PrintString "SetNewWindTarget")
      (bind _asbp_ghost_wind_target (Utilities|Casting|CastToBP_GhostWindTarget (Variables|Default|GetNextWindTarget)))
      (Variables|/Script/Engine.PrimitiveComponent|SetbGenerateOverlapEvents (Variables|BP_GhostWindTarget_C|GetCollisionSphere _asbp_ghost_wind_target) true)
      (Variables|/Script/Engine.PrimitiveComponent|SetbGenerateOverlapEvents (Variables|Default|GetSphere) false))))

(event EventBeginPlay
  (Variables|Default|SetCollisionSphere (Variables|Default|GetSphere)))

(fn ConstructionScript)