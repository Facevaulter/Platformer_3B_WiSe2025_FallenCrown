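; Trigger volume that shows an on-screen tutorial when the player's BP_SkeletonKing enters its box.
; A TutorialTypeEnum variable selects the movement, jump or sprint widget, which is passed to the player's BP_Hud through ShowTutorialText.
; Leaving the box calls HideTutorial on the same HUD.
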(event OnComponentBeginOverlap(Box)
  (params (OverlappedComponent :type Primitive%20Component%20Object%20Reference) (OtherActor :type Actor%20Object%20Reference) (OtherComp :type Primitive%20Component%20Object%20Reference) (OtherBodyIndex :type Integer) (bFromSweep :type Boolean) (SweepResult :type Hit%20Result%20Structure%20%28by%20ref%29))
  (Utilities|Casting|CastToBP_SkeletonKing OtherActor)
  (switch Utilities|FlowControl|Switch|SwitchonETutorialType (Variables|Default|GetTutorialTypeEnum)
    (:NewEnumerator0
      (bind _asbp_hud (Utilities|Casting|CastToBP_Hud (HUD|GetHUD (Game|GetPlayerController 0))))
      (Default|ShowTutorialText _asbp_hud "/Game/UI/Widgets/WBP_MovementTut.WBP_MovementTut_C"))
    (:NewEnumerator1
      (bind _asbp_hud_2 (Utilities|Casting|CastToBP_Hud (HUD|GetHUD (Game|GetPlayerController 0))))
      (Default|ShowTutorialText _asbp_hud_2 "/Game/UI/Widgets/WBP_JumpTutorial.WBP_JumpTutorial_C"))
    (:NewEnumerator3
      (bind _asbp_hud_3 (Utilities|Casting|CastToBP_Hud (HUD|GetHUD (Game|GetPlayerController 0))))
      (Default|ShowTutorialText _asbp_hud_3 "/Game/UI/Widgets/WBP_SprintTut.WBP_SprintTut_C"))))

(event OnComponentEndOverlap(Box)
  (params (OverlappedComponent :type Primitive%20Component%20Object%20Reference) (OtherActor :type Actor%20Object%20Reference) (OtherComp :type Primitive%20Component%20Object%20Reference) (OtherBodyIndex :type Integer))
  (Utilities|Casting|CastToBP_SkeletonKing OtherActor)
  (bind _asbp_hud (Utilities|Casting|CastToBP_Hud (HUD|GetHUD (Game|GetPlayerController 0))))
  (Default|HideTutorial _asbp_hud))

(event EventBeginPlay)

(event Collision|EventActorBeginOverlap
  (params (OtherActor :type Actor%20Object%20Reference)))

(event EventTick
  (params (DeltaSeconds :type Float%20%28single-precision%29)))

(fn ConstructionScript)