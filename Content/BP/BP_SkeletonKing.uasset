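; Player character for the Skeleton King, handling Enhanced Input movement, sphere-overlap interaction, spawn-point respawns and a toggleable ghost form.
; Ghosting swaps crown, cape and body material, toggles the ghost realm and crossfades the soundtrack.
; A recursive delay loop drains energy, fading ghost material opacity through dynamic instances, and pickups replenish it.
; Exiting or depletion starts a timeline cooldown shown on the HUD; the endgame event grants infinite energy.
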(event Custom|Respawn
  (bind _returnvalue (Game|GetPlayerCameraManager 0))
  ;[0.15 0.15 0.15 0.5] Respawn
  (Utilities|FlowControl|DoOnce false
    (:Completed
      (Audio|PlaySound2D "/Game/Audio/Sfx/DeathSFX.DeathSFX" 1.0 1.0 0.0 0 0)
      (Input|DisableInput (Game|GetPlayerController 0))
      (CameraFades|StartCameraFade :self _returnvalue :ToAlpha 1.0 :Duration 0.3 :bHoldWhenFinished true)
      (Utilities|FlowControl|Delay 2.0)
      (if (Variables|GhostAbility|GetGhosted)
        (CallFunction|EndGhostAbility))
      (CallFunction|TeleporttoSpawn)
      (CameraFades|StartCameraFade :self _returnvalue :FromAlpha 1.0 :Duration 1.5 :bShouldFadeAudio true)
      (Input|EnableInput (Game|GetPlayerController 0)))))

(event Custom|StartGhostAbilityCooldown
  ;[0 0.8073 0.5186 0.5] GhostAbility Cooldown
  (CallFunction|WidgetCooldownSetAbilityonCooldown)
  (bind _ghostabilitycooldown (Timeline|CooldownGhostAbility PlayFromStart)
    (:Update
      (CallFunction|WidgetCooldownUpdateCooldown _ghostabilitycooldown))
    (:Finished
      (Variables|GhostAbility|SetAbilityReady true)
      (CallFunction|WidgetCooldownAbilityReady)
      (bind _asbp_hud (Utilities|Casting|CastToBP_Hud (HUD|GetHUD (Game|GetPlayerController 0))))
      (Default|ClearCooldownCounter (Variables|/Game/UI/BP_Hud.BP_Hud_C|GetAbilityCooldownWidget _asbp_hud)))))

(event Custom|EndGameGhostform
  (Variables|Default|SetInfiniteGhostEnergy true)
  ;[0 0.8073 0.5186 0.5] Start Ghost Ability
  (if (Variables|GhostAbility|GetGhosted)
    (CallFunction|EndGhostAbility)
    (elif (Variables|GhostAbility|GetAbilityReady)
      (Variables|GhostAbility|SetAbilityReady false)
      (CallFunction|ToggleVisibilityGhostItems)
      (CallFunction|WidgetCooldownAbilityToggle true)
      (CallFunction|BeginnEnergieLoss)
      (Default|CallToggleGhostRealm)
      (CallFunction|ResetEndGhostAbility)
      (CallFunction|ToggleSoundtrack)
      (Rendering|Material|SetMaterial (Variables|Character|GetMesh) 1 "/Game/Material/GhostMat/MI_GhostMat.MI_GhostMat"))))

(event Custom|InputDeviceChanged
  (params (bNewInputType :type ECommonInputType%20Enum :default "MouseAndKeyboard"))
  (bind _asbp_game_instance (Utilities|Casting|CastToBP_GameInstance (Game|GetGameInstance)))
  (switch Utilities|FlowControl|Switch|SwitchonECommonInputType bNewInputType
    (:MouseAndKeyboard
      (Variables|/Game/BP/BP_GameInstance.BP_GameInstance_C|SetKeyboard%20Input _asbp_game_instance true))
    (:Gamepad
      (Variables|/Game/BP/BP_GameInstance.BP_GameInstance_C|SetKeyboard%20Input _asbp_game_instance false))))

(event Custom|EndGhostAbility
  ;[0 0.8073 0.5186 0.5] End Ghost Ability
  (Variables|GhostAbility|SetGhostEnerhyLoopClosed true)
  (CallFunction|ToggleVisibilityGhostItems)
  (CallFunction|WidgetCooldownAbilityToggle false)
  (CallFunction|StartGhostAbilityCooldown)
  (Default|CallToggleGhostRealm)
  (Default|CallRespawnGhostEnergy)
  (CallFunction|ToggleSoundtrack)
  (Rendering|Material|SetMaterial (Variables|Character|GetMesh) 1 "/Game/Material/MI_InvisibleTranslucent.MI_InvisibleTranslucent"))

(event Custom|EnergyLossLoop
  ;[0 0.8073 0.5186 0.5] Energy Loss Loop
  (if (not (Variables|GhostAbility|GetGhostEnerhyLoopClosed))
    (if (> (Variables|GhostAbility|GetEnergy) 0.0)
      (Utilities|FlowControl|Delay (Variables|GhostAbility|GetEnergyReducTikTime))
      (if (Variables|Default|GetInfiniteGhostEnergy)
        _
        (else
          (Variables|GhostAbility|SetEnergy (- (Variables|GhostAbility|GetEnergy) (Variables|GhostAbility|GetEnergyLossOnTick)))))
      (CallFunction|EnergyLossLoop)
      (bind _newtrack_0 (Timeline|GhostMatOpacityLerpTimeline PlayFromStart)
        (:Update
          (CallFunction|SetGhostCrownandCapeOpacitytoEnergyPerc _newtrack_0)))
      (else
        (Utilities|FlowControl|DoOnce false
          (:Completed
            (CallFunction|EndGhostAbility)))))))

(event Custom|GetGhostEnergy
  (params (A :type Float%20%28double-precision%29))
  ;[0 0.8073 0.5186 0.5] Energy Gain
  (if (< (+ A (Variables|GhostAbility|GetEnergy)) (Variables|GhostAbility|GetMaxEnergy))
    (Variables|GhostAbility|SetEnergy (+ A (Variables|GhostAbility|GetEnergy)))
    (bind _newtrack_0 (Timeline|GainEnergyTimeline PlayFromStart)
      (:Update
        (Rendering|Material|SetScalarParameterValue (Variables|Default|GetMID%20GhostMat%20Cape) "ExponentIn" (- (Variables|Default|GetScalarParaBaseValueExponent) _newtrack_0) :!class /Script/Engine.MaterialInstanceDynamic)))
    (else
      (Variables|GhostAbility|SetEnergy (Variables|GhostAbility|GetMaxEnergy))
      (Timeline|GainEnergyTimeline PlayFromStart))))

(event Custom|Reset%20Respawn
  (bind _returnvalue (Game|GetPlayerCameraManager 0))
  ;[0.15 0.15 0.15 0.5] Respawn
  (Utilities|FlowControl|DoOnce false) ; enters at Reset
)

(event Custom|Reset%20End%20Ghost%20Ability
  ;[0 0.8073 0.5186 0.5] Energy Loss Loop
  (Utilities|FlowControl|DoOnce false) ; enters at Reset
)

(event Custom|ToggleSoundtrack
  (if (Variables|GhostAbility|GetGhosted)
    (bind _newtrack_0 (Timeline|SoundTrackFadeTimeline Play)
      (:Update
        (Audio|Parameter|SetFloatParameter (Variables|Default|GetSC_GameSoundTrack) "SoundTrackFade" _newtrack_0 :!class /Script/Engine.AudioComponent)))
    (else
      (Timeline|SoundTrackFadeTimeline Reverse))))

(event Custom|BeginnEnergieLoss
  ;[0 0.8073 0.5186 0.5] Energy Loss Loop
  (Variables|GhostAbility|SetGhostEnerhyLoopClosed false)
  (Variables|GhostAbility|SetEnergy (Variables|GhostAbility|GetStartingEnergy))
  (if (> (Variables|GhostAbility|GetEnergy) 0.0)
    (Utilities|FlowControl|Delay (Variables|GhostAbility|GetEnergyReducTikTime))
    (if (Variables|Default|GetInfiniteGhostEnergy)
      _
      (else
        (Variables|GhostAbility|SetEnergy (- (Variables|GhostAbility|GetEnergy) (Variables|GhostAbility|GetEnergyLossOnTick)))))
    (CallFunction|EnergyLossLoop)
    (bind _newtrack_0 (Timeline|GhostMatOpacityLerpTimeline PlayFromStart)
      (:Update
        (CallFunction|SetGhostCrownandCapeOpacitytoEnergyPerc _newtrack_0)))
    (else
      (Utilities|FlowControl|DoOnce false
        (:Completed
          (CallFunction|EndGhostAbility))))))

(event Input|EnhancedActionEvents|EnhancedInputActionIA_Move
  (params (ActionValue :type Vector%202D%20Structure) (ElapsedSeconds :type Float%20%28double-precision%29) (TriggeredSeconds :type Float%20%28double-precision%29) (InputAction :type Input%20Action%20Object%20Reference :default "/Game/Input/Actions/IA_Move.IA_Move"))
  ;[0.01455 0.15 0.01847 0.5] Input
  (CallFunction|MoveinLocalDir (.x ActionValue) (.y ActionValue)))

(event Input|EnhancedActionEvents|EnhancedInputActionIA_Look
  (params (ActionValue :type Vector%202D%20Structure) (ElapsedSeconds :type Float%20%28double-precision%29) (TriggeredSeconds :type Float%20%28double-precision%29) (InputAction :type Input%20Action%20Object%20Reference :default "/Game/Input/Actions/IA_Look.IA_Look"))
  ;[0.01455 0.15 0.01847 0.5] Input
  (bind _asbp_game_instance (Utilities|Casting|CastToBP_GameInstance (Game|GetGameInstance)))
  (Pawn|Input|AddControllerYawInput (* (Variables|/Game/BP/BP_FallenCrownVolumeSettingSavegame.BP_FallenCrownVolumeSettingSavegame_C|GetLookSpeedMultyplier (Variables|/Game/BP/BP_GameInstance.BP_GameInstance_C|GetVolumeSettingSaveGame _asbp_game_instance)) (.x ActionValue)))
  (Pawn|Input|AddControllerPitchInput (* (Variables|/Game/BP/BP_FallenCrownVolumeSettingSavegame.BP_FallenCrownVolumeSettingSavegame_C|GetLookSpeedMultyplier (Variables|/Game/BP/BP_GameInstance.BP_GameInstance_C|GetVolumeSettingSaveGame _asbp_game_instance)) (.y ActionValue))))

(event Input|EnhancedActionEvents|EnhancedInputActionIA_Jump
  (params (ActionValue :type Boolean) (ElapsedSeconds :type Float%20%28double-precision%29) (TriggeredSeconds :type Float%20%28double-precision%29) (InputAction :type Input%20Action%20Object%20Reference :default "/Game/Input/Actions/IA_Jump.IA_Jump"))
  ;[0.01455 0.15 0.01847 0.5] Input
  (:Triggered
    (if (not (Variables|Movement|GetBunnyhopBreak))
      (Character|Jump)
      (Variables|Movement|SetBunnyhopBreak true)))
  (:Completed
    (Character|StopJumping)
    (Variables|Movement|SetBunnyhopBreak false)))

(event Input|EnhancedActionEvents|EnhancedInputActionIA_Sprint
  (params (ActionValue :type Boolean) (ElapsedSeconds :type Float%20%28double-precision%29) (TriggeredSeconds :type Float%20%28double-precision%29) (InputAction :type Input%20Action%20Object%20Reference :default "/Game/Input/Actions/IA_Sprint.IA_Sprint"))
  ;[0.01455 0.15 0.01847 0.5] Input
  (:Triggered
    (Variables|Movement|SetWants%20to%20sprint true))
  (:Completed
    (Variables|Movement|SetWants%20to%20sprint false)))

(event Input|EnhancedActionEvents|EnhancedInputActionIA_Interact
  (params (ActionValue :type Boolean) (ElapsedSeconds :type Float%20%28double-precision%29) (TriggeredSeconds :type Float%20%28double-precision%29) (InputAction :type Input%20Action%20Object%20Reference :default "/Game/Input/Actions/IA_Interact.IA_Interact"))
  (bind _interactsphere (Variables|Default|GetInteractSphere))
  ;[0.01455 0.15 0.01847 0.5] Input
  (bind _outactors (Collision|SphereOverlapActors (Transformation|GetWorldLocation _interactsphere) (Components|Sphere|GetScaledSphereRadius _interactsphere) (Utilities|Array|MakeArray "ObjectTypeQuery1" "ObjectTypeQuery2" "ObjectTypeQuery3") 0 (Utilities|Array|MakeArray self)))
  (for _array_element _outactors
    (if (Utilities|DoesObjectImplementInterface _array_element "/Game/BP/Interfaces/InteractableInteraface.InteractableInteraface_C")
      (Class|InteractableInteraface|Interact(Message) _array_element))))

(event Input|EnhancedActionEvents|EnhancedInputActionIA_Pause
  (params (ActionValue :type Boolean) (ElapsedSeconds :type Float%20%28double-precision%29) (TriggeredSeconds :type Float%20%28double-precision%29) (InputAction :type Input%20Action%20Object%20Reference :default "/Game/Input/Actions/IA_Pause.IA_Pause"))
  ;[0.01455 0.15 0.01847 0.5] Input
  (bind _asbp_hud (Utilities|Casting|CastToBP_Hud (HUD|GetHUD (Game|GetPlayerController 0))))
  (Default|Pause _asbp_hud))

(event Input|EnhancedActionEvents|EnhancedInputActionIA_ToggleGhostAbility
  (params (ActionValue :type Boolean) (ElapsedSeconds :type Float%20%28double-precision%29) (TriggeredSeconds :type Float%20%28double-precision%29) (InputAction :type Input%20Action%20Object%20Reference :default "/Game/Input/Actions/IA_ToggleGhostAbility.IA_ToggleGhostAbility"))
  ;[0 0.8073 0.5186 0.5] Start Ghost Ability
  (if (Variables|GhostAbility|GetGhosted)
    (CallFunction|EndGhostAbility)
    (elif (Variables|GhostAbility|GetAbilityReady)
      (Variables|GhostAbility|SetAbilityReady false)
      (CallFunction|ToggleVisibilityGhostItems)
      (CallFunction|WidgetCooldownAbilityToggle true)
      (CallFunction|BeginnEnergieLoss)
      (Default|CallToggleGhostRealm)
      (CallFunction|ResetEndGhostAbility)
      (CallFunction|ToggleSoundtrack)
      (Rendering|Material|SetMaterial (Variables|Character|GetMesh) 1 "/Game/Material/GhostMat/MI_GhostMat.MI_GhostMat"))))

(event EventBeginPlay
  ;[0.15 0.15 0.15 0.5] BeginPlay
  (Utilities|FlowControl|Sequence
    (:then_0
      (CallFunction|TeleporttoSpawn))
    (:then_1
      (Input|AddMappingContext (PlayerController|LocalPlayerSubsystems|GetEnhancedInputLocalPlayerSubsystem (Game|GetPlayerController 0)) "/Game/Input/IMC_Default.IMC_Default" 0 "(bIgnoreAllPressedKeysUntilRelease=True,bForceImmediately=False,bNotifyUserSettings=False)"))
    (:then_2
      (Components|SkinnedMesh|SetLeaderPoseComponent (Variables|Default|GetGhostCrown_GRT) (Variables|Character|GetMesh) false false))
    (:then_3
      (Components|Timeline|SetPlayRate (Variables|Default|GetCooldownGhostAbility) 1.0)
      (Components|Timeline|SetPlayRate (Variables|Default|GetGhostMatOpacityLerpTimeline) (/ 1.0 (Variables|GhostAbility|GetEnergyReducTikTime))))
    (:then_4
      (Audio|Components|Audio|Play (Variables|Default|GetSC_GameSoundTrack) 0.0)
      (Components|Timeline|SetPlayRate (Variables|Default|GetSoundTrackFadeTimeline) (/ 1.0 (Variables|Default|GetSoundTrackFadeTimelinePlayrate))))
    (:then_5
      (bind _returnvalue (Rendering|Material|CreateDynamicMaterialInstance (Variables|Default|GetGhostCape_GRT) 0 0 "None" :!class /Script/Engine.PrimitiveComponent))
      (Variables|Default|SetMID%20GhostMat%20Cape _returnvalue)
      (bind _returnvalue_2 (Rendering|Material|CreateDynamicMaterialInstance (Variables|Default|GetGhostCrown_GRT) 0 0 "None" :!class /Script/Engine.PrimitiveComponent))
      (Variables|Default|SetMID%20GhostMat%20Crown _returnvalue_2)
      (bind _returnvalue_3 (Rendering|Material|GetScalarParameterValue (Variables|Default|GetMID%20GhostMat%20Cape) "ExponentIn" :!class /Script/Engine.MaterialInstanceDynamic))
      (Variables|Default|SetScalarParaBaseValueExponent _returnvalue_3)
      (bind _returnvalue_4 (Rendering|Material|GetScalarParameterValue (Variables|Default|GetMID%20GhostMat%20Cape) "OuterColorOpacity" :!class /Script/Engine.MaterialInstanceDynamic))
      (Variables|Default|SetScalarParaBaseValueOuterOp _returnvalue_4)
      (bind _returnvalue_5 (Rendering|Material|GetScalarParameterValue (Variables|Default|GetMID%20GhostMat%20Cape) "InnerColorOpacity" :!class /Script/Engine.MaterialInstanceDynamic))
      (Variables|Default|SetScalarParaBaseValueInnerOp _returnvalue_5)
      (Components|Timeline|SetPlayRate (Variables|Default|GetGainEnergyTimeline) (/ 1.0 (Variables|Default|GetGainEnergyTimelinePlayrate))))
    (:then_6
      (EventDispatchers|BindEventtoOnInputMethodChanged (PlayerController|LocalPlayerSubsystems|GetCommonInputSubsystem (Game|GetPlayerController 0)) (delegate Custom|InputDeviceChanged)))))

(event EventTick
  (params (DeltaSeconds :type Float%20%28single-precision%29))
  (bind _charactermovement (Variables|Character|GetCharacterMovement))
  (Utilities|FlowControl|Sequence
    (:then_0
      ;[0.15 0.15 0.15 0.5] SprintCheck
      (if (and (Variables|Movement|GetWants%20to%20sprint) (AI|Components|NavMovement|IsMovingonGround (Variables|Character|GetCharacterMovement)))
        (Variables|/Script/Engine.CharacterMovementComponent|SetMaxWalkSpeed _charactermovement (Variables|Movement|GetSprintSpeed))
        (else
          (Variables|/Script/Engine.CharacterMovementComponent|SetMaxWalkSpeed _charactermovement (Variables|Movement|GetWalkSpeed)))))
    (:then_1
      (if (Variables|GhostAbility|GetGhosted)
        (Transformation|SetWorldRotation (Variables|Default|GetPivot_GhostWind) (Math|Rotator|FindLookatRotation (Transformation|GetActorLocation) (Variables|Default|GetGhostWIndTarget)) false false)))
    (:then_2
      (if (and (Variables|Default|GetIsAirborne) (not (AI|Components|NavMovement|IsFalling (Variables|Character|GetCharacterMovement))))
        (Audio|PlaySound2D "/Game/Audio/Sfx/LandingBoneRattleSFX.LandingBoneRattleSFX" 0.1 1.0 0.0 0 0)
        (Variables|Default|SetIsAirborne false)
        (elif (and (AI|Components|NavMovement|IsFalling (Variables|Character|GetCharacterMovement)) (not (Variables|Default|GetIsAirborne)))
          (Variables|Default|SetIsAirborne true))))))

(fn ConstructionScript
  (Variables|/Script/Engine.CharacterMovementComponent|SetMaxWalkSpeed (Variables|Character|GetCharacterMovement) (Variables|Movement|GetWalkSpeed)))

(fn MoveinLocalDir
  (params (LocalDirection_X :type Float%20%28double-precision%29) (LocalDirection_Y :type Float%20%28double-precision%29))
  (bind _camera (Variables|Default|GetCamera))
  (bind _returnvalue (Transformation|GetWorldTransform _camera))
  (Pawn|Input|AddMovementInput (Math|Transform|TransformDirection (Math|Transform|MakeTransform (.location _returnvalue) (Math|Rotator|MakeRotator 0.0 0.0 (.yaw (.rotation _returnvalue))) (.scale _returnvalue)) (Math|Vector|MakeVector LocalDirection_X LocalDirection_Y 0.0)) 1.0 false))

(fn TeleporttoSpawn
  (bind _asbp_game_instance (Utilities|Casting|CastToBP_GameInstance (Game|GetGameInstance))
    (:then
      (if (.HasValidPlayerSpawnTransform (Default|TryGetPlayerSpawnTransform _asbp_game_instance))
        (Transformation|SetActorLocationAndRotation (.location (.PlayerSpawnTransform (Default|TryGetPlayerSpawnTransform _asbp_game_instance))) (.rotation (.PlayerSpawnTransform (Default|TryGetPlayerSpawnTransform _asbp_game_instance))))
        (CallFunction|ResetRespawn)))
    (:CastFailed
      (Development|PrintString "WRONG GAME INSTANCE" true true "(R=1.000000,G=0.019690,B=0.000000,A=1.000000)" 5.0))))

(fn ToggleVisibilityGhostItems
  (Development|SetHiddeninGame (Variables|Default|GetGhostCrown_GRT) (Variables|GhostAbility|GetGhosted) false)
  (Development|SetHiddeninGame (Variables|Default|GetOldCrown_GRT) (not (Variables|GhostAbility|GetGhosted)) false)
  (Development|PrintText "Vidsibility Toggled" true true "(R=1.000000,G=0.000000,B=0.011742,A=1.000000)")
  (Variables|GhostAbility|SetGhosted (not (Variables|GhostAbility|GetGhosted))))

(fn WidgetCooldownUpdateCooldown
  (params (A :type Float%20%28double-precision%29))
  (bind _asbp_hud (Utilities|Casting|CastToBP_Hud (HUD|GetHUD (Game|GetPlayerController 0))))
  (Default|UpdateCooldown (Variables|/Game/UI/BP_Hud.BP_Hud_C|GetAbilityCooldownWidget _asbp_hud) (Math|Float|Truncate A)))

(fn WidgetCooldownAbilityReady
  (bind _asbp_hud (Utilities|Casting|CastToBP_Hud (HUD|GetHUD (Game|GetPlayerController 0))))
  (Default|AbilityCastReady (Variables|/Game/UI/BP_Hud.BP_Hud_C|GetAbilityCooldownWidget _asbp_hud)))

(fn WidgetCooldownSetAbilityonCooldown
  (bind _asbp_hud (Utilities|Casting|CastToBP_Hud (HUD|GetHUD (Game|GetPlayerController 0))))
  (Default|AbilityonCooldown (Variables|/Game/UI/BP_Hud.BP_Hud_C|GetAbilityCooldownWidget _asbp_hud)))

(fn WidgetCooldownAbilityToggle
  (params (Condition :type Boolean))
  (bind _asbp_hud (Utilities|Casting|CastToBP_Hud (HUD|GetHUD (Game|GetPlayerController 0))))
  (Default|AbilityActiveToggle (Variables|/Game/UI/BP_Hud.BP_Hud_C|GetAbilityCooldownWidget _asbp_hud) Condition))

(fn SetGhostCrownandCapeOpacitytoEnergyPerc
  (params (Alpha :type Float%20%28double-precision%29))
  (bind _energylossontick (Variables|GhostAbility|GetEnergyLossOnTick))
  (bind _energy (Variables|GhostAbility|GetEnergy))
  (bind _maxenergy (Variables|GhostAbility|GetMaxEnergy))
  (bind _returnvalue (+ _energy _energylossontick))
  (bind _returnvalue_2 (/ _maxenergy 2.0))
  (bind _returnvalue_3 (Math|Float|Lerp _energy _returnvalue Alpha))
  (bind _returnvalue_4 (/ _returnvalue_3 _returnvalue_2))
  (Rendering|Material|SetScalarParameterValue (Variables|Default|GetMID%20GhostMat%20Cape) "OuterColorOpacity" (* _returnvalue_4 (Variables|Default|GetScalarParaBaseValueOuterOp)) :!class /Script/Engine.MaterialInstanceDynamic)
  (Rendering|Material|SetScalarParameterValue (Variables|Default|GetMID%20GhostMat%20Cape) "InnerColorOpacity" (* _returnvalue_4 (Variables|Default|GetScalarParaBaseValueInnerOp)) :!class /Script/Engine.MaterialInstanceDynamic))