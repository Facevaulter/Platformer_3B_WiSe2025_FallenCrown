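; BP_GameEnd is a trigger box that ends the game when BP_SkeletonKing overlaps it.
; It sets FinishedGame on the game instance's VolumeSettingSaveGame and calls SaveEndgame to save it.
; It fades the camera and audio out over a short delay, then sets ShowCredits on the game instance and opens MainMenu.
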(event OnComponentBeginOverlap(Box)
  (params (OverlappedComponent :type Primitive%20Component%20Object%20Reference) (OtherActor :type Actor%20Object%20Reference) (OtherComp :type Primitive%20Component%20Object%20Reference) (OtherBodyIndex :type Integer) (bFromSweep :type Boolean) (SweepResult :type Hit%20Result%20Structure%20%28by%20ref%29))
  (Utilities|Casting|CastToBP_SkeletonKing OtherActor)
  (bind _asbp_game_instance (Utilities|Casting|CastToBP_GameInstance (Game|GetGameInstance)))
  (Variables|/Game/BP/BP_FallenCrownVolumeSettingSavegame.BP_FallenCrownVolumeSettingSavegame_C|SetFinishedGame (Variables|/Game/BP/BP_GameInstance.BP_GameInstance_C|GetVolumeSettingSaveGame _asbp_game_instance) true)
  (bind _asbp_game_instance_2 (Utilities|Casting|CastToBP_GameInstance (Game|GetGameInstance)))
  (Default|SaveEndgame _asbp_game_instance_2)
  (CameraFades|StartCameraFade :self (Game|GetPlayerCameraManager 0) :ToAlpha 1.0 :Duration 2.0 :bShouldFadeAudio true :bHoldWhenFinished true)
  (Utilities|FlowControl|Delay 2.0)
  (bind _asbp_game_instance_3 (Utilities|Casting|CastToBP_GameInstance (Game|GetGameInstance)))
  (Variables|/Game/BP/BP_GameInstance.BP_GameInstance_C|SetShowCredits _asbp_game_instance_3 true)
  (Game|OpenLevel(byObjectReference) "/Game/Maps/MainMenu.MainMenu"))

(fn ConstructionScript)