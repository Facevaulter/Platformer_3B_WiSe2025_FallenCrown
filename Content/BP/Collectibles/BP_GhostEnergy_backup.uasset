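; BP_GhostEnergy is a collectible that grants ghost energy to the BP_SkeletonKing player character.
; Self-restarting timelines spin the pivot and bob the sphere while idle.
; On BeginPlay it registers its root and sphere in SpookyAsset's ghost visibility and trigger arrays.
; The first SkeletonKing overlap awards the energy, changes the spin rate, stops the bob and plays a shoot-up timeline that destroys the actor when finished.
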(event OnComponentBeginOverlap(Sphere)
  (params (OverlappedComponent :type Primitive%20Component%20Object%20Reference) (OtherActor :type Actor%20Object%20Reference) (OtherComp :type Primitive%20Component%20Object%20Reference) (OtherBodyIndex :type Integer) (bFromSweep :type Boolean) (SweepResult :type Hit%20Result%20Structure%20%28by%20ref%29))
  ;[0.15 0.15 0.15 0.5] Collision Detection
  (Utilities|Casting|CastToBP_SkeletonKing OtherActor)
  (Utilities|FlowControl|DoOnce false
    (:Completed
      (CallFunction|GetCollected))))

(event Custom|GetCollected
  (bind _asbp_skeleton_king (Utilities|Casting|CastToBP_SkeletonKing (Game|GetPlayerCharacter 0)))
  (Default|GetGhostEnergy _asbp_skeleton_king (Variables|Default|GetEnergyGainValue))
  ;[0.15 0.15 0.15 0.5] Collection Effekt
  (Components|Timeline|SetPlayRate (Variables|Default|GetSpinTImeline) (* (Variables|Animation|GetSpinSpeed) 3.0))
  (CallFunction|StopBop)
  (CallFunction|ShootUp))

(event Custom|Spin
  ;[0.15 0.15 0.15 0.5] Idle Animation
  (bind _spinpercent (Timeline|SpinTImeline PlayFromStart)
    (:Update
      (Transformation|SetRelativeRotation (Variables|Default|GetPivot) (Math|Rotator|MakeRotator 0.0 0.0 (* _spinpercent 3.6e+02)) false false))
    (:Finished
      (CallFunction|Spin))))

(event Custom|Bop
  ;[0.15 0.15 0.15 0.5] Idle Animation
  (bind _normalbop (Timeline|BopTimeline PlayFromStart)
    (:Update
      (Transformation|SetRelativeLocation (Variables|Default|GetSphere) (Math|Vector|MakeVector 0.0 0.0 (* _normalbop (Variables|Animation|GetBopHeight))) false false))
    (:Finished
      (CallFunction|Bop))))

(event Custom|StopBop
  ;[0.15 0.15 0.15 0.5] Idle Animation
  (bind _normalbop (Timeline|BopTimeline Stop)
    (:Update
      (Transformation|SetRelativeLocation (Variables|Default|GetSphere) (Math|Vector|MakeVector 0.0 0.0 (* _normalbop (Variables|Animation|GetBopHeight))) false false))
    (:Finished
      (CallFunction|Bop))))

(event Custom|ShootUp
  ;[0.15 0.15 0.15 0.5] PickUpAnimation
  (bind _shootup (Timeline|ShootUpTimeline PlayFromStart)
    (:Update
      (Transformation|SetRelativeLocation (Variables|Default|GetPivot) (Math|Vector|MakeVector 0.0 0.0 (* _shootup (Variables|Animation|GetShootUpHeight))) false false))
    (:Finished
      (Actor|DestroyActor))))

(event EventBeginPlay
  (bind _spookyasset (Variables|Default|GetSpookyAsset))
  ;[0.15 0.15 0.15 0.5] Initial setup
  (Components|Timeline|SetPlayRate (Variables|Default|GetSpinTImeline) (/ 1.0 (Variables|Animation|GetSpinSpeed)))
  (Components|Timeline|SetPlayRate (Variables|Default|GetBopTimeline) (/ 1.0 (Variables|Animation|GetBopSpeed)))
  (Components|Timeline|SetPlayRate (Variables|Default|GetShootUpTimeline) (/ 1.0 (Variables|Animation|GetShootUpSpeed)))
  (CallFunction|Spin)
  (CallFunction|Bop)
  (Utilities|Array|Add (Variables|/Game/BP/Components/SpookyAsset_Component.SpookyAsset_Component_C|GetGhostActorArray_Visibility _spookyasset) (Variables|Default|GetDefaultSceneRoot))
  (Utilities|Array|Add (Variables|/Game/BP/Components/SpookyAsset_Component.SpookyAsset_Component_C|GetGhostActorArray_TriggerSphere _spookyasset) (Variables|Default|GetSphere)))

(fn ConstructionScript)