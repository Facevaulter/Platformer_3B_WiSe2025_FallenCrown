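; BP_Coin1 is a collectible coin that idles with a spin and bop, then counts toward the HUD when a BP_Character overlaps it.
; Timelines scaled by speed variables drive the animation, with spin and bop restarting themselves to loop.
; On the first valid Sphere overlap, it updates the HUD's collectibles widget, changes the spin rate and stops the bop.
; A shoot-up timeline then lifts the Pivot and destroys the actor when finished.
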(event OnComponentBeginOverlap(Sphere)
  (params (OverlappedComponent :type Primitive%20Component%20Object%20Reference) (OtherActor :type Actor%20Object%20Reference) (OtherComp :type Primitive%20Component%20Object%20Reference) (OtherBodyIndex :type Integer) (bFromSweep :type Boolean) (SweepResult :type Hit%20Result%20Structure%20%28by%20ref%29))
  ;[0.15 0.15 0.15 0.5] Collision Detection
  (Utilities|Casting|CastToBP_Character OtherActor)
  (Utilities|FlowControl|DoOnce false
    (:Completed
      (CallFunction|GetCollected))))

(event Custom|GetCollected
  ;[0.15 0.15 0.15 0.5] Increase in UI
  (bind _asbp_hud (Utilities|Casting|CastToBP_Hud (HUD|GetHUD (Game|GetPlayerController 0))))
  (Default|CollectCoin (Variables|/Game/UI/BP_Hud.BP_Hud_C|GetCollectiblesWidget _asbp_hud) 1)
  ;[0.15 0.15 0.15 0.5] Collection Effekt
  (Components|Timeline|SetPlayRate (Variables|Default|GetSpinTImeline) (* (Variables|Default|GetSpinSpeed) 3.0))
  (CallFunction|StopBop)
  (CallFunction|ShootUp))

(event Custom|Spin
  ;[0.15 0.15 0.15 0.5] Idle Animation
  (bind _spinpercent (Timeline|SpinTImeline PlayFromStart)
    (:Update
      (Transformation|SetRelativeRotation (Variables|Default|GetPivot) (Math|Rotator|MakeRotator 0.0 0.0 (* _spinpercent 3.6e+02)) false false))
    (:Finished
      (CallFunction|Spin))))

(event Custom|Bop
  ;[0.15 0.15 0.15 0.5] Idle Animation
  (bind _normalbop (Timeline|BopTimeline PlayFromStart)
    (:Update
      (Transformation|SetRelativeLocation (Variables|Default|GetSphere) (Math|Vector|MakeVector 0.0 0.0 (* _normalbop (Variables|Default|GetBopHeight))) false false))
    (:Finished
      (CallFunction|Bop))))

(event Custom|StopBop
  ;[0.15 0.15 0.15 0.5] Idle Animation
  (bind _normalbop (Timeline|BopTimeline Stop)
    (:Update
      (Transformation|SetRelativeLocation (Variables|Default|GetSphere) (Math|Vector|MakeVector 0.0 0.0 (* _normalbop (Variables|Default|GetBopHeight))) false false))
    (:Finished
      (CallFunction|Bop))))

(event Custom|ShootUp
  ;[0.15 0.15 0.15 0.5] PickUpAnimation
  (bind _shootup (Timeline|ShootUpTimeline PlayFromStart)
    (:Update
      (Transformation|SetRelativeLocation (Variables|Default|GetPivot) (Math|Vector|MakeVector 0.0 0.0 (* _shootup (Variables|Default|GetShootUpHeight))) false false))
    (:Finished
      (Actor|DestroyActor))))

(event EventBeginPlay
  ;[0.15 0.15 0.15 0.5] Initial setup
  (Components|Timeline|SetPlayRate (Variables|Default|GetSpinTImeline) (/ 1.0 (Variables|Default|GetSpinSpeed)))
  (Components|Timeline|SetPlayRate (Variables|Default|GetBopTimeline) (/ 1.0 (Variables|Default|GetBopSpeed)))
  (Components|Timeline|SetPlayRate (Variables|Default|GetShootUpTimeline) (/ 1.0 (Variables|Default|GetShootUpSpeed)))
  (CallFunction|Spin)
  (CallFunction|Bop))

(fn ConstructionScript)