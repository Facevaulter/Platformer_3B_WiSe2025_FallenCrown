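; Ghost energy pickup that idles with looping spin and bob timelines on its Pivot and registers its root in SpookyAsset's ghost visibility array.
; GetCollected, which nothing in this graph calls, grants energy to the player's BP_SkeletonKing and plays a pickup sound.
; It then changes the spin rate, stops the bob and shoots the pivot upward, destroying the actor when that timeline finishes.
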(event Custom|GetCollected
  (Utilities|FlowControl|Sequence
    (:then_0
      (bind _asbp_skeleton_king (Utilities|Casting|CastToBP_SkeletonKing (Game|GetPlayerCharacter 0)))
      (Default|GetGhostEnergy _asbp_skeleton_king (Variables|Default|GetEnergyGainValue)))
    (:then_1
      (Audio|PlaySoundatLocation "/Game/Audio/Sfx/EnergyPickupSFX.EnergyPickupSFX" (Transformation|GetActorLocation) "0, 0, 0" 0.5 1.0 0.0 0 0 0 0))
    (:then_2
      ;[0.15 0.15 0.15 0.5] Collection Effekt
      (Components|Timeline|SetPlayRate (Variables|Default|GetSpinTImeline) (* (Variables|Animation|GetSpinSpeed) 3.0))
      (CallFunction|StopBop)
      (CallFunction|ShootUp))))

(event Custom|Spin
  ;[0.15 0.15 0.15 0.5] Idle Animation
  (bind _spinpercent (Timeline|SpinTImeline PlayFromStart)
    (:Update
      (Transformation|SetRelativeRotation (Variables|Default|GetPivot) (Math|Rotator|MakeRotator 0.0 0.0 (* _spinpercent 3.6e+02)) false false))
    (:Finished
      (CallFunction|Spin))))

(event Custom|Bop
  ;[0.15 0.15 0.15 0.5] Idle Animation
  (bind _normalbop (Timeline|BopTimeline PlayFromStart)
    (:Update
      (Transformation|SetRelativeLocation (Variables|Default|GetPivot) (Math|Vector|MakeVector 0.0 0.0 (* _normalbop (Variables|Animation|GetBopHeight))) false false))
    (:Finished
      (CallFunction|Bop))))

(event Custom|StopBop
  ;[0.15 0.15 0.15 0.5] Idle Animation
  (bind _normalbop (Timeline|BopTimeline Stop)
    (:Update
      (Transformation|SetRelativeLocation (Variables|Default|GetPivot) (Math|Vector|MakeVector 0.0 0.0 (* _normalbop (Variables|Animation|GetBopHeight))) false false))
    (:Finished
      (CallFunction|Bop))))

(event Custom|ShootUp
  ;[0.15 0.15 0.15 0.5] PickUpAnimation
  (bind _shootup (Timeline|ShootUpTimeline PlayFromStart)
    (:Update
      (Transformation|SetRelativeLocation (Variables|Default|GetPivot) (Math|Vector|MakeVector 0.0 0.0 (* _shootup (Variables|Animation|GetShootUpHeight))) false false))
    (:Finished
      (Actor|DestroyActor))))

(event EventBeginPlay
  ;[0.15 0.15 0.15 0.5] Initial setup
  (Components|Timeline|SetPlayRate (Variables|Default|GetSpinTImeline) (/ 1.0 (Variables|Animation|GetSpinSpeed)))
  (Components|Timeline|SetPlayRate (Variables|Default|GetBopTimeline) (/ 1.0 (Variables|Animation|GetBopSpeed)))
  (Components|Timeline|SetPlayRate (Variables|Default|GetShootUpTimeline) (/ 1.0 (Variables|Animation|GetShootUpSpeed)))
  (CallFunction|Spin)
  (CallFunction|Bop)
  (Utilities|Array|Add (Variables|/Game/BP/Components/SpookyAsset_Component.SpookyAsset_Component_C|GetGhostActorArray_Visibility (Variables|Default|GetSpookyAsset)) (Variables|Default|GetDefaultSceneRoot)))

(fn ConstructionScript)